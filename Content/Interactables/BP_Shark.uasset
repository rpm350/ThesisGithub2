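; BP_Shark is an interactable shark that squeaks when the Perform input action is pressed.
; Each press sets ShowPressedButton, which appears to drive a pressed UI button, and release clears it.
; A random integer below NumSounds picks the sound: zero plays Squeak1 and any other value plays Squeak2.
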(event EventBeginPlay
  (|CallParentFunction) ; This node is disabled and will not be called.\nDrag off pins to build functionality.
)

(event Collision|EventActorBeginOverlap
  (params (OtherActor :type Actor%20Object%20Reference)))

(event EventTick
  (params (DeltaSeconds :type Float%20%28single-precision%29))
  (|CallParentFunction DeltaSeconds) ; This node is disabled and will not be called.\nDrag off pins to build functionality.
)

(event Input|ActionEvents|InputActionPerform
  (params (Key :type Key%20Structure))
  (:Pressed
    ;[1 1 1] Show the pressed UI button?
    (Variables|Default|SetshowPressedButton true)
    (if (== (Math|Random|RandomInteger (Variables|Default|GetnumSounds)) 0)
      (Audio|Components|Audio|Play (Variables|Default|Getsqueak1) 0.0)
      (else
        (Audio|Components|Audio|Play (Variables|Default|Getsqueak2) 0.0))))
  (:Released
    (Variables|Default|SetshowPressedButton false)))

(fn ConstructionScript
  (|CallParentFunction))