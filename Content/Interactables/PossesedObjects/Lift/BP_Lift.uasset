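; BP_Lift is a possessable lift vehicle with throttle, steering and handbrake input, plus a timeline that raises and lowers its mesh on Up/Down.
; Holding SearchMode outlines transferable BallTemplate and BP_Lift actors through custom depth and line-traces along the camera to select one.
; Transfer blends the view to the selection, then possesses it.
; Wheels overlapping a source BP_Puddle spawn capped puddle trails on Tick, spaced by X/Z movement checks.
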(event OnComponentBeginOverlap(backRIghtWheel)
  (params (OverlappedComponent :type Primitive%20Component%20Object%20Reference) (OtherActor :type Actor%20Object%20Reference) (OtherComp :type Primitive%20Component%20Object%20Reference) (OtherBodyIndex :type Integer) (bFromSweep :type Boolean) (SweepResult :type Hit%20Result%20Structure%20%28by%20ref%29))
  (bind _asbp_puddle (Utilities|Casting|CastToBP_Puddle OtherActor))
  (if (Variables|/Game/Interactables/BP_Puddle.BP_Puddle_C|GetcanTrail _asbp_puddle)
    (if (Variables|/Game/Interactables/BP_Puddle.BP_Puddle_C|GetsourcePuddle _asbp_puddle)
      (if (or (>= (Variables|Default|GetBRTimer) (Variables|Default|GetspawnPuddleMax)) (== (Variables|Default|GetBRTimer) 0))
        (Variables|Default|SettrackingBR true)
        (Variables|Default|SetBRTimer 0)))))

(event OnComponentBeginOverlap(frontRightWheel)
  (params (OverlappedComponent :type Primitive%20Component%20Object%20Reference) (OtherActor :type Actor%20Object%20Reference) (OtherComp :type Primitive%20Component%20Object%20Reference) (OtherBodyIndex :type Integer) (bFromSweep :type Boolean) (SweepResult :type Hit%20Result%20Structure%20%28by%20ref%29))
  (bind _asbp_puddle (Utilities|Casting|CastToBP_Puddle OtherActor))
  (Development|PrintString (Utilities|String|ToString(Integer) (Variables|Default|GetFRTimer)))
  (if (Variables|/Game/Interactables/BP_Puddle.BP_Puddle_C|GetcanTrail _asbp_puddle)
    (if (Variables|/Game/Interactables/BP_Puddle.BP_Puddle_C|GetsourcePuddle _asbp_puddle)
      (if (or (>= (Variables|Default|GetFRTimer) (Variables|Default|GetspawnPuddleMax)) (== (Variables|Default|GetFRTimer) 0))
        (Development|PrintString (Utilities|String|ToString(Boolean) false))
        (Variables|Default|SettrackingFR true)
        (Variables|Default|SetFRTimer 0)))))

(event OnComponentBeginOverlap(backLeftWheel)
  (params (OverlappedComponent :type Primitive%20Component%20Object%20Reference) (OtherActor :type Actor%20Object%20Reference) (OtherComp :type Primitive%20Component%20Object%20Reference) (OtherBodyIndex :type Integer) (bFromSweep :type Boolean) (SweepResult :type Hit%20Result%20Structure%20%28by%20ref%29))
  (bind _asbp_puddle (Utilities|Casting|CastToBP_Puddle OtherActor))
  (if (Variables|/Game/Interactables/BP_Puddle.BP_Puddle_C|GetcanTrail _asbp_puddle)
    (if (Variables|/Game/Interactables/BP_Puddle.BP_Puddle_C|GetsourcePuddle _asbp_puddle)
      (if (or (>= (Variables|Default|GetBLTimer) (Variables|Default|GetspawnPuddleMax)) (== (Variables|Default|GetBLTimer) 0))
        (Variables|Default|SettrackingBL true)
        (Variables|Default|SetBLTimer 0)))))

(event OnComponentBeginOverlap(frontLeftWheel)
  (params (OverlappedComponent :type Primitive%20Component%20Object%20Reference) (OtherActor :type Actor%20Object%20Reference) (OtherComp :type Primitive%20Component%20Object%20Reference) (OtherBodyIndex :type Integer) (bFromSweep :type Boolean) (SweepResult :type Hit%20Result%20Structure%20%28by%20ref%29))
  (bind _asbp_puddle (Utilities|Casting|CastToBP_Puddle OtherActor))
  (if (Variables|/Game/Interactables/BP_Puddle.BP_Puddle_C|GetcanTrail _asbp_puddle)
    (if (Variables|/Game/Interactables/BP_Puddle.BP_Puddle_C|GetsourcePuddle _asbp_puddle)
      (if (or (>= (Variables|Default|GetFLTimer) (Variables|Default|GetspawnPuddleMax)) (== (Variables|Default|GetFLTimer) 0))
        (Variables|Default|SettrackingFL true)
        (Variables|Default|SetFLTimer 0)))))

(event Custom|highlightTransferableObjects
  ;[1 1 1] Highlight
  (Utilities|IsValid (Variables|Default|GetselectedPawn)
    (:Is%20Valid
      (bind _asball_template (Utilities|Casting|CastToBallTemplate (Variables|Default|GetselectedPawn))
        (:then
          (Rendering|Material|SetMaterial (Variables|/Game/Interactables/PossesedObjects/BallTemplate.BallTemplate_C|GetStaticMesh _asball_template) 0 (Variables|/Game/Interactables/PossesedObjects/BallTemplate.BallTemplate_C|GetmydefaultMaterial _asball_template)))
        (:CastFailed
          (bind _asbp_lift (Utilities|Casting|CastToBP_Lift (Variables|Default|GetselectedPawn)))
          (Rendering|Material|SetMaterial (Variables|BP_Lift_C|GetStaticMesh _asbp_lift) 0 (Variables|BP_Lift_C|GetmydefaultMaterial _asbp_lift))))
      (Variables|Default|SetselectedPawn 0))
    (:Is%20Not%20Valid
      _))
  (Variables|Default|SetsearchMode true)
  (for _array_element (Variables|Default|GettransferableClasses)
    (bind _outactors (Actor|GetAllActorsOfClass _array_element))
    (for _array_element_2 _outactors
      (bind _asball_template_2 (Utilities|Casting|CastToBallTemplate _array_element_2)
        (:then
          (if (!= self _asball_template_2)
            (Rendering|SetRenderCustomDepth (Variables|/Game/Interactables/PossesedObjects/BallTemplate.BallTemplate_C|GetStaticMesh _asball_template_2) true)))
        (:CastFailed
          (bind _asbp_lift_2 (Utilities|Casting|CastToBP_Lift _array_element_2))
          (if (!= self _asbp_lift_2)
            (Rendering|SetRenderCustomDepth (Variables|BP_Lift_C|GetStaticMesh _asbp_lift_2) true)))))))

(event Custom|unHighlight
  (bind _selectedpawn (Variables|Default|GetselectedPawn))
  ;[1 1 1] Unhighlight
  (Variables|Default|SetsearchMode false)
  (for _array_element (Variables|Default|GettransferableClasses)
    (bind _outactors (Actor|GetAllActorsOfClass _array_element))
    (for _array_element_2 _outactors
      (if (!= self _array_element_2)
        (bind _asball_template (Utilities|Casting|CastToBallTemplate _selectedpawn)
          (:then
            (if (not (== _asball_template _array_element_2))
              (bind _asball_template_2 (Utilities|Casting|CastToBallTemplate _array_element_2 :!label _label)
                (:then
                  (Rendering|Material|SetMaterial (Variables|/Game/Interactables/PossesedObjects/BallTemplate.BallTemplate_C|GetStaticMesh _asball_template_2) 0 (Variables|/Game/Interactables/PossesedObjects/BallTemplate.BallTemplate_C|GetmydefaultMaterial _asball_template_2))
                  (Rendering|SetRenderCustomDepth (Variables|/Game/Interactables/PossesedObjects/BallTemplate.BallTemplate_C|GetStaticMesh _asball_template_2) false))
                (:CastFailed
                  (bind _asbp_lift (Utilities|Casting|CastToBP_Lift _array_element_2))
                  (Rendering|Material|SetMaterial (Variables|BP_Lift_C|GetStaticMesh _asbp_lift) 0 (Variables|BP_Lift_C|GetmydefaultMaterial _asbp_lift))
                  (Rendering|SetRenderCustomDepth (Variables|BP_Lift_C|GetStaticMesh _asbp_lift) false)))))
          (:CastFailed
            (bind _asbp_lift_2 (Utilities|Casting|CastToBP_Lift _selectedpawn)
              (:then
                (if (not (== _array_element_2 _asbp_lift_2))
                  (goto _label)))
              (:CastFailed
                (goto _label)))))))))

(event Custom|CustomEvent
  ;[1 1 1] Setup each transferrable with its Individual Materials
  (Rendering|Material|SetMaterial (Variables|Default|GetStaticMesh) 0 (Variables|Default|GetmyTexture))
  ;[1 1 1] Set up static obj with rotating camera
  (Variables|Default|SetmeshRot (Transformation|GetWorldRotation (Variables|Default|GetStaticMesh))))

(event EventTick
  (params (DeltaSeconds :type Float%20%28single-precision%29))
  (bind _frontrightwheel (Variables|Default|GetfrontRightWheel))
  (bind _staticmesh (Variables|Default|GetStaticMesh))
  (bind _backrightwheel (Variables|Default|GetbackRIghtWheel))
  (bind _backleftwheel (Variables|Default|GetbackLeftWheel))
  (bind _frontleftwheel (Variables|Default|GetfrontLeftWheel))
  (bind _returnvalue (Transformation|GetWorldLocation _staticmesh))
  (bind _returnvalue_2 (Transformation|GetWorldLocation _frontrightwheel))
  (bind _returnvalue_3 (Transformation|GetWorldLocation _backrightwheel))
  (bind _returnvalue_4 (Transformation|GetWorldLocation _backleftwheel))
  (bind _returnvalue_5 (Transformation|GetWorldLocation _frontleftwheel))
  ;[1 1 1] Check if need to trail the puddle
  (if (Variables|Default|GettrackingBR)
    (if (<= (Variables|Default|GetBRTimer) (Variables|Default|GetspawnPuddleMax))
      (bind _movedfarenoughtospawn (CallFunction|AbsVal _returnvalue_3 (Variables|Default|GetBRprevLoc)))
      (if _movedfarenoughtospawn
        (Game|SpawnActorfromClass "/Game/Interactables/BP_Puddle.BP_Puddle_C" (Math|Transform|MakeTransform (Transformation|GetWorldLocation (Variables|Default|GetbackRIghtWheel))) "Undefined" 0 0)
        (Variables|Default|SetBRprevLoc _returnvalue_3)
        (Variables|Default|SetBRTimer (+ (Variables|Default|GetBRTimer) 1)))))
  (if (Variables|Default|GettrackingBL)
    (if (<= (Variables|Default|GetBLTimer) (Variables|Default|GetspawnPuddleMax))
      (bind _movedfarenoughtospawn_2 (CallFunction|AbsVal _returnvalue_4 (Variables|Default|GetBLprevLoc)))
      (if _movedfarenoughtospawn_2
        (Game|SpawnActorfromClass "/Game/Interactables/BP_Puddle.BP_Puddle_C" (Math|Transform|MakeTransform (Transformation|GetWorldLocation (Variables|Default|GetbackLeftWheel))) "Undefined" 0 0)
        (Variables|Default|SetBLprevLoc _returnvalue_4)
        (Variables|Default|SetBLTimer (+ (Variables|Default|GetFLTimer) 1)))))
  (if (Variables|Default|GettrackingFR)
    (if (<= (Variables|Default|GetFRTimer) (Variables|Default|GetspawnPuddleMax))
      (bind _movedfarenoughtospawn_3 (CallFunction|AbsVal _returnvalue_2 (Variables|Default|GetFRprevLoc)))
      (if _movedfarenoughtospawn_3
        (Game|SpawnActorfromClass "/Game/Interactables/BP_Puddle.BP_Puddle_C" (Math|Transform|MakeTransform (Transformation|GetWorldLocation (Variables|Default|GetfrontRightWheel))) "Undefined" 0 0)
        (Variables|Default|SetFRprevLoc _returnvalue_2)
        (Variables|Default|SetFRTimer (+ (Variables|Default|GetFRTimer) 1)))))
  (if (Variables|Default|GettrackingFL)
    (if (<= (Variables|Default|GetFLTimer) (Variables|Default|GetspawnPuddleMax))
      (bind _movedfarenoughtospawn_4 (CallFunction|AbsVal _returnvalue_5 (Variables|Default|GetFLprevLoc)))
      (if _movedfarenoughtospawn_4
        (Game|SpawnActorfromClass "/Game/Interactables/BP_Puddle.BP_Puddle_C" (Math|Transform|MakeTransform (Transformation|GetWorldLocation (Variables|Default|GetfrontLeftWheel))) "Undefined" 0 0)
        (Variables|Default|SetFLprevLoc _returnvalue_5)
        (Variables|Default|SetFLTimer (+ (Variables|Default|GetFLTimer) 1)))))
  ;[1 1 1] Search mode?
  (if (Variables|Default|GetsearchMode)
    ;[1 1 1] Ray Cast
    (bind (_outhit _returnvalue_6) (Collision|LineTraceByChannel _returnvalue (+ _returnvalue (* (Transformation|GetActorForwardVector (Game|GetPlayerCameraManager 0)) (Variables|Default|GetmaxLookDistance))) "TraceTypeQuery1" false 0 "ForOneFrame" true "(R=0.000000,G=0.907450,B=1.000000,A=1.000000)" "(R=0.000000,G=1.000000,B=0.000000,A=1.000000)" 0.01))
    (if _returnvalue_6
      ;[1 1 1] Hit success - STATIC OBJECT (BALL TEMPLATE)
      (bind _asball_template (Utilities|Casting|CastToBallTemplate (.HitActor (Collision|BreakHitResult _outhit)))
        (:then
          (if (not (== (Variables|Default|GetselectedPawn) _asball_template))
            (bind _output_get (Variables|Default|SetselectedPawn _asball_template))
            (Variables|Default|SetIs_Ready true)
            (Rendering|Material|SetMaterial (Variables|/Game/Interactables/PossesedObjects/BallTemplate.BallTemplate_C|GetStaticMesh _asball_template) 0 "/Game/Materials/highlightMaterial2.highlightMaterial2")
            (bind _outactors (Actor|GetAllActorsOfClass "/Game/Interactables/PossesedObjects/BallTemplate.BallTemplate_C"))
            (for _array_element _outactors
              (if (!= _array_element _output_get)
                (if (!= self _array_element)
                  (Rendering|Material|SetMaterial (Variables|/Game/Interactables/PossesedObjects/BallTemplate.BallTemplate_C|GetStaticMesh _array_element) 0 (Variables|/Game/Interactables/PossesedObjects/BallTemplate.BallTemplate_C|GetmydefaultMaterial _array_element)))))))
        (:CastFailed
          ;[1 1 1] Hit success - VEHICLE (BP_LIFT)
          (bind _asbp_lift (Utilities|Casting|CastToBP_Lift (.HitActor (Collision|BreakHitResult _outhit)))
            (:then
              (if (not (== _asbp_lift (Variables|Default|GetselectedPawn)))
                (bind _output_get_2 (Variables|Default|SetselectedPawn _asbp_lift))
                (Variables|Default|SetIs_Ready true)
                (Rendering|Material|SetMaterial (Variables|BP_Lift_C|GetStaticMesh _asbp_lift) 0 "/Game/Materials/highlightMaterial2.highlightMaterial2")
                (bind _outactors_2 (Actor|GetAllActorsOfClass "BP_Lift_C"))
                (for _array_element_2 _outactors_2
                  (if (!= _array_element_2 _output_get_2)
                    (if (!= self _array_element_2)
                      (Rendering|Material|SetMaterial (Variables|BP_Lift_C|GetStaticMesh _array_element_2) 0 (Variables|BP_Lift_C|GetmydefaultMaterial _array_element_2)))))))
            (:CastFailed
              ;[1 1 1] Hit failure - deselect
              (bind _asball_template_2 (Utilities|Casting|CastToBallTemplate (Variables|Default|GetselectedPawn))
                (:then
                  (Rendering|Material|SetMaterial (Variables|/Game/Interactables/PossesedObjects/BallTemplate.BallTemplate_C|GetStaticMesh _asball_template_2) 0 (Variables|/Game/Interactables/PossesedObjects/BallTemplate.BallTemplate_C|GetmydefaultMaterial _asball_template_2))
                  (Variables|Default|SetselectedPawn 0)
                  (Variables|Default|SetIs_Ready false))
                (:CastFailed
                  (bind _asbp_lift_2 (Utilities|Casting|CastToBP_Lift (Variables|Default|GetselectedPawn)))
                  (Rendering|Material|SetMaterial (Variables|BP_Lift_C|GetStaticMesh _asbp_lift_2) 0 (Variables|BP_Lift_C|GetmydefaultMaterial _asbp_lift_2))
                  (Variables|Default|SetselectedPawn 0)
                  (Variables|Default|SetIs_Ready false))))))))))

(event EventBeginPlay
  (Variables|Default|SetBRprevLoc (Transformation|GetWorldLocation (Variables|Default|GetbackRIghtWheel)))
  (Variables|Default|SetFRprevLoc (Transformation|GetWorldLocation (Variables|Default|GetfrontRightWheel)))
  (Variables|Default|SetBLprevLoc (Transformation|GetWorldLocation (Variables|Default|GetbackLeftWheel)))
  (Variables|Default|SetFLprevLoc (Transformation|GetWorldLocation (Variables|Default|GetfrontLeftWheel))))

(event Input|ActionEvents|InputActionTransfer
  (params (Key :type Key%20Structure))
  (bind _staticmesh (Variables|Default|GetStaticMesh))
  ;[1 1 1] Possess/Transfer
  (:Pressed
    (if (Variables|Default|GetsearchMode)
      _
      (else
        _))
    (if (Variables|Default|GetIs_Ready)
      (Utilities|IsValid (Variables|Default|GetselectedPawn)
        (:Is%20Valid
          (bind _asball_template (Utilities|Casting|CastToBallTemplate (Variables|Default|GetselectedPawn))
            (:then
              (Rendering|Material|SetMaterial (Variables|/Game/Interactables/PossesedObjects/BallTemplate.BallTemplate_C|GetStaticMesh _asball_template) 0 (Variables|/Game/Interactables/PossesedObjects/BallTemplate.BallTemplate_C|GetmydefaultMaterial _asball_template)))
            (:CastFailed
              (bind _asbp_lift (Utilities|Casting|CastToBP_Lift (Variables|Default|GetselectedPawn)))
              (Rendering|Material|SetMaterial (Variables|BP_Lift_C|GetStaticMesh _asbp_lift) 0 (Variables|BP_Lift_C|GetmydefaultMaterial _asbp_lift))))
          (Components|Movement|StopMovementImmediately (Variables|Default|GetVehicleMovement))
          (CallFunction|UnHighlight)
          ;[1 1 1] Camera Transition to Possess
          (Game|Player|SetViewTargetwithBlend (Game|GetPlayerController 0) (Variables|Default|GetselectedPawn) 1.5 "VTBlend_Cubic" 0.0 false)
          (Utilities|FlowControl|Delay 2.0)
          (Pawn|Possess (Game|GetPlayerController 0) (Variables|Default|GetselectedPawn))
          (Rendering|Material|SetMaterial _staticmesh 0 (Variables|Default|GetmydefaultMaterial))
          (Rendering|SetRenderCustomDepth _staticmesh false)
          (Variables|/Game/ThirdPersonBP/Blueprints/HUD.HUD_C|SetcurrentPosses (Variables|Default|GetHUD) (Variables|Default|GetselectedPawn))
          (Variables|Default|SetselectedPawn 0))))))

(event Input|ActionEvents|InputActionSearchMode
  (params (Key :type Key%20Structure))
  ;[1 1 1] Trigger Search Mode
  (:Pressed
    (CallFunction|HighlightTransferableObjects))
  (:Released
    (CallFunction|UnHighlight)))

(event Input|ActionEvents|InputActionJump
  (params (Key :type Key%20Structure))
  (bind _vehiclemovement (Variables|Default|GetVehicleMovement))
  ;[1 1 1] Movement Control
  (:Pressed
    (Class|WheeledVehicleMovementComponent|SetHandbrakeInput _vehiclemovement true))
  (:Released
    (Class|WheeledVehicleMovementComponent|SetHandbrakeInput _vehiclemovement false)))

(event Input|AxisEvents|InputAxisLookUp
  (params (AxisValue :type Float%20%28single-precision%29))
  ;[1 1 1] Movement Control
  (Pawn|Input|AddControllerPitchInput AxisValue))

(event Input|AxisEvents|InputAxisTurn
  (params (AxisValue :type Float%20%28single-precision%29))
  ;[1 1 1] Movement Control
  (Pawn|Input|AddControllerYawInput AxisValue))

(event Input|AxisEvents|InputAxisMoveForward
  (params (AxisValue :type Float%20%28single-precision%29))
  ;[1 1 1] Movement Control
  (Class|WheeledVehicleMovementComponent|SetThrottleInput (Variables|Default|GetVehicleMovement) AxisValue))

(event Input|AxisEvents|InputAxisMoveRight
  (params (AxisValue :type Float%20%28single-precision%29))
  ;[1 1 1] Movement Control
  (Class|WheeledVehicleMovementComponent|SetSteeringInput (Variables|Default|GetVehicleMovement) AxisValue))

(event Input|KeyboardEvents|Up
  (params (Key :type Key%20Structure))
  ;[1 1 1] Raise Lift
  (:Pressed
    (bind _newtrack_0 (Timeline|LiftTime Play)
      (:Update
        (Transformation|SetRelativeLocation (Variables|Default|GetStaticMesh) (Math|Vector|Lerp(Vector) (Variables|Default|GetstartPoint) (Variables|Default|GetendPoint) _newtrack_0) false false)))))

(event Input|KeyboardEvents|Down
  (params (Key :type Key%20Structure))
  ;[1 1 1] Raise Lift
  (:Pressed
    (bind _newtrack_0 (Timeline|LiftTime Reverse)
      (:Update
        (Transformation|SetRelativeLocation (Variables|Default|GetStaticMesh) (Math|Vector|Lerp(Vector) (Variables|Default|GetstartPoint) (Variables|Default|GetendPoint) _newtrack_0) false false)))))

(fn ConstructionScript)

(fn AbsVal
  (params (currentPos :type Vector) (prevPos :type Vector))
  (bind (_x _y _z) (Math|Vector|BreakVector currentPos))
  (bind (_x_2 _y_2 _z_2) (Math|Vector|BreakVector prevPos))
  (bind _puddlediam (Variables|Default|GetpuddleDiam))
  (Variables|Default|SetabsVal_x false)
  (Variables|Default|SetabsVal_z false)
  (if (< _x (+ _x_2 _puddlediam))
    ;[1 1 1] Change is too small
    (Variables|Default|SetabsVal_x false)
    (if (> _x (- _x_2 _puddlediam))
      (Variables|Default|SetabsVal_x false)
      (if (< _z (+ _z_2 _puddlediam))
        (Variables|Default|SetabsVal_z false)
        (if (> _z (- _z_2 _puddlediam))
          (Variables|Default|SetabsVal_z false)
          (return false)
          (else
            (Variables|Default|SetabsVal_z true)))
        (else
          (Variables|Default|SetabsVal_z true)))
      (return true)
      (else
        (Variables|Default|SetabsVal_x true)))
    (else
      (Variables|Default|SetabsVal_x true)))
  (return true))