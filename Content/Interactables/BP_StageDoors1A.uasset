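; BP_StageDoors1A is a stage door interactable that rotates its Door1A component on Tick.
; A branch selects a lerp toward an open or closed rotation, but its condition is fixed false, so only the closed path runs.
; That path lerps from DefaultSceneRoot's rotation rather than the door's own, using DeltaSeconds as alpha, so it does not accumulate toward the closed position as the open path would.
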(event EventTick
  (params (DeltaSeconds :type Float%20%28single-precision%29))
  (bind _returnvalue (* DeltaSeconds 1.0))
  (|CallParentFunction DeltaSeconds)
  (if false
    (Transformation|SetRelativeRotation (Variables|Default|GetDoor1A) (Math|Rotator|Lerp(Rotator) (.Rotation (Math|Transform|BreakTransform (Transformation|GetRelativeTransform (Variables|Default|GetDoor1A)))) (Variables|Default|GetDoorOpenPosition) _returnvalue) false false)
    (else
      (Transformation|SetRelativeRotation (Variables|Default|GetDoor1A) (Math|Rotator|Lerp(Rotator) (.Rotation (Math|Transform|BreakTransform (Transformation|GetRelativeTransform (Variables|Default|GetDefaultSceneRoot)))) (Variables|Default|GetDoorClosedPosition) _returnvalue) false false))))

(fn ConstructionScript)