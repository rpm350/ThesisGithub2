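; Actor component that auto-aims a Pawn by turning its control rotation toward a target found with a camera-forward box trace.
; BeginPlay caches the camera and control-rotation spring arm or camera; StartTrace picks the target and enables Tick.
; Tick steers toward it with optional smoothing and clamped free-look offsets.
; Aiming ends on EndTrace, lost line of sight or sustained input, with delegates reporting start, end and failure.
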(event Custom|StartTrace
  ;[0 0.05 1] Start the tracing. First check if our component references are valid and if they are then continue with tracing.
  (Utilities|IsValid (Variables|Default|GetStartLookAtComponent)
    (:Is%20Valid
      (Utilities|IsValid (Variables|Default|GetCameraComponent)
        (:Is%20Valid
          (bind _breturnvalue (Private|InternalTrace (Variables|Internal|GetIgnoreActors)))
          (Variables|Internal|SetbIsTracingActive _breturnvalue)
          (Utilities|FlowControl|Sequence
            (:then_0
              (Variables|Internal|SetbUseManualStartLocation (Math|Vector|NotEqual(Vector) (Variables|Internal|GetStartLocation) "0, 0, 0" 0.0001))
              (Variables|Internal|SetbUseManualTargetLocation (Math|Vector|NotEqual(Vector) (Variables|Internal|GetTargetLocation) "0, 0, 0" 0.0001)))
            (:then_1
              (Components|Tick|SetComponentTickEnabled (Variables|Internal|GetbIsTracingActive)))))
        (:Is%20Not%20Valid
          (Private|InternalTraceFailed "Camera Component Invalid!"))))
    (:Is%20Not%20Valid
      (Private|InternalTraceFailed "Start Look At Component Invalid!"))))

(event Custom|EndTrace
  ;[0 0.05 1] End the tracing. Set Hit Target to null and call Aim Ended delegate.
  (Variables|Internal|SetbIsTracingActive false)
  (Variables|Internal|SetHitTarget 0)
  (Default|CallOnAutoAimEnded))

(event Custom|TryCancelAutoAimFromInput
  (params (InAxisValue :type Float%20%28single-precision%29%20%28by%20ref%29))
  ;[0 0.05 1] Try to cancel auto aiming when given input axis is above the threshold.
  (if (Variables|Internal|GetbIsTracingActive)
    (if (!= InAxisValue 0.0)
      (Utilities|FlowControl|Sequence
        (:then_0
          (Utilities|FlowControl|DoOnce false :!label _label
            (:Completed
              (Variables|Internal|SetLastTime (Utilities|Time|GetGameTimeinSeconds)))))
        (:then_1
          (if (>= (- (Utilities|Time|GetGameTimeinSeconds) (Variables|Internal|GetLastTime)) (Variables|AutoAimComponent|GetInputTimeToCancel))
            (CallFunction|EndTrace))))
      (else
        (goto _label Reset)))))

(event Custom|FreeLook
  (params (PitchAxis :type Float%20%28single-precision%29%20%28by%20ref%29) (YawAxis :type Float%20%28single-precision%29%20%28by%20ref%29))
  (bind _freelookdistance (Variables|AutoAimComponent|FreeLook|GetFreeLookDistance))
  (bind _freelookdistance_2 (Variables|AutoAimComponent|FreeLook|GetFreeLookDistance))
  ;[0 0 0] UPDATE 1.1 - Free look lets the player aim away within a certain distance. NOTE: This works better with Gamepad input.
  (if (Variables|Internal|GetbIsTracingActive)
    (if (Variables|AutoAimComponent|FreeLook|GetbEnableFreeLooking)
      (Utilities|FlowControl|Sequence
        (:then_0
          (if (!= YawAxis 0.0)
            (Variables|Internal|SetCurrentFreeLookDistance_Yaw (Math|Float|Clamp(Float) (+ (Variables|Internal|GetCurrentFreeLookDistance_Yaw) YawAxis) (* _freelookdistance_2 -1.0) _freelookdistance_2))
            (else
              (Variables|Internal|SetCurrentFreeLookDistance_Yaw 0.0))))
        (:then_1
          (if (!= PitchAxis 0.0)
            (Variables|Internal|SetCurrentFreeLookDistance_Pitch (Math|Float|Clamp(Float) (+ (Variables|Internal|GetCurrentFreeLookDistance_Pitch) (Math|Float|SelectFloat PitchAxis (* PitchAxis -1.0) (Variables|AutoAimComponent|FreeLook|GetbInvertFreeLookPitch))) (* _freelookdistance -1.0) _freelookdistance))
            (else
              (Variables|Internal|SetCurrentFreeLookDistance_Pitch 0.0))))))
    (else
      (Variables|Internal|SetCurrentFreeLookDistance_Yaw 0.0)
      (Variables|Internal|SetCurrentFreeLookDistance_Pitch 0.0))))

(event EventBeginPlay
  ;[0 0.05 1] At begin play loop through all the children components of root component and find SprinArmComponent and CameraComponent. If they are available and they use pawn control rotation then save them as references.
  (bind _array_element (Utilities|Array|ForEachLoopwithBreak (Components|GetChildrenComponents (VehicleSound|GetRootComponent (Components|GetOwner)) true) :!label _label)
    (:LoopBody
      (bind _asspring_arm_component (Utilities|Casting|CastToSpringArmComponent _array_element)
        (:then
          (if (Variables|/Script/Engine.SpringArmComponent|GetbUsePawnControlRotation _asspring_arm_component)
            (Variables|Default|SetStartLookAtComponent _asspring_arm_component)))
        (:CastFailed
          (bind _ascamera_component (Utilities|Casting|CastToCameraComponent _array_element))
          (bind _output_get (Variables|Default|SetCameraComponent _ascamera_component))
          (if (Variables|/Script/Engine.CameraComponent|GetbUsePawnControlRotation _output_get)
            (Variables|Default|SetStartLookAtComponent (Variables|Default|GetCameraComponent))
            (goto _label Break)
            (else
              (goto _label Break))))))
    (:Completed
      (Utilities|IsValid (Variables|Default|GetStartLookAtComponent)
        (:Is%20Valid
          (bind _aspawn (Utilities|Casting|CastToPawn (Components|GetOwner (Variables|Default|GetStartLookAtComponent))))
          (Variables|Internal|SetOwnerPawn _aspawn))
        (:Is%20Not%20Valid
          (Private|InternalTraceFailed "Owner Pawn failed to set!"))))))

(event EventTick
  (params (DeltaSeconds :type Float%20%28single-precision%29))
  (bind _ownerpawn (Variables|Internal|GetOwnerPawn))
  (bind _returnvalue (Pawn|GetController _ownerpawn))
  (bind _returnvalue_2 (Pawn|GetControlRotation _returnvalue :!class /Script/Engine.Controller))
  ;[0 0.05 1] Check if we are tracing in this frame.
  (if (Variables|Internal|GetbIsTracingActive)
    ;;[0 0 0] UPDATE 1.1 - Every frame check if we have LoS to our target. If not then gracefully end auto aiming.
    (if (Private|InternalHasLineOfSight)
      ;;[0.1 1 0] Still tracing? Make sure our owner pawn is valid and set control rotation using Find Look at Rotation node.
      (Utilities|IsValid _ownerpawn
        (:Is%20Valid
          (Variables|Internal|SetCurrentLookAtRotation (Private|InternalGetLookatRotation))
          (Variables|Internal|SetCurrentControlRotation (select (Variables|AutoAimComponent|GetbUseSmoothAiming) (Math|Interpolation|RInterpTo _returnvalue_2 (Variables|Internal|GetCurrentLookAtRotation) DeltaSeconds (Variables|AutoAimComponent|GetInterpSpeed)) (Variables|Internal|GetCurrentLookAtRotation)))
          (Pawn|SetControlRotation _returnvalue (Math|Rotator|SelectRotator (Math|Rotator|SelectRotator (Math|Interpolation|RInterpTo _returnvalue_2 (Math|Rotator|MakeRotator (.Roll (Math|Rotator|BreakRotator (Variables|Internal|GetCurrentLookAtRotation))) (+ (.Pitch (Math|Rotator|BreakRotator (Variables|Internal|GetCurrentLookAtRotation))) (Variables|Internal|GetCurrentFreeLookDistance_Pitch)) (+ (.Yaw (Math|Rotator|BreakRotator (Variables|Internal|GetCurrentLookAtRotation))) (Variables|Internal|GetCurrentFreeLookDistance_Yaw))) DeltaSeconds (Variables|AutoAimComponent|GetInterpSpeed)) (Math|Rotator|MakeRotator (.Roll (Math|Rotator|BreakRotator (Variables|Internal|GetCurrentLookAtRotation))) (+ (.Pitch (Math|Rotator|BreakRotator (Variables|Internal|GetCurrentLookAtRotation))) (Variables|Internal|GetCurrentFreeLookDistance_Pitch)) (+ (.Yaw (Math|Rotator|BreakRotator (Variables|Internal|GetCurrentLookAtRotation))) (Variables|Internal|GetCurrentFreeLookDistance_Yaw))) (Variables|AutoAimComponent|GetbUseSmoothAiming)) (Variables|Internal|GetCurrentControlRotation) (Variables|AutoAimComponent|FreeLook|GetbEnableFreeLooking)))
          (Private|InternalShowDebugTraceLine))
        (:Is%20Not%20Valid
          (Private|InternalTraceFailed "AutoAimComponents owner was not Pawn.")))
      (else
        (CallFunction|EndTrace)))
    (else
      ;;[1 0.05 0] Not Tracing? Then disable ticking for this component.
      (Components|Tick|SetComponentTickEnabled false))))

(fn InternalTrace
  (params (ActorsToIgnore :type Array%20of%20Actor%20Object%20References))
  (bind _cameracomponent (Variables|Default|GetCameraComponent))
  (Utilities|FlowControl|Sequence
    (:then_0
      (Variables|Internal|SetCameraLocation (Transformation|GetWorldLocation _cameracomponent))
      (Variables|Internal|SetForwardVector (Math|Vector|GetForwardVector _cameracomponent))
      (Utilities|FlowControl|Sequence
        (:then_0
          (if (or (Variables|Debug|GetbDrawTrace) (Variables|Debug|GetbDrawTraceHitSphere))
            (Rendering|Debug|FlushPersistentDebugLines)))
        (:then_1
          (bind _output_get (LocalVariables|SetLocal_TraceEndLocation (+ (Variables|Internal|GetCameraLocation) (* (Variables|Internal|GetForwardVector) (Variables|AutoAimComponent|GetTraceDistance)))))
          (bind (_outhit _returnvalue) (Class|KismetSystemLibrary|BoxTraceSingleforObjects (Variables|Internal|GetCameraLocation) _output_get (Math|Conversions|ToVector(Float) (Variables|AutoAimComponent|GetTraceSize)) (Math|Conversions|RotationFromXVector (Variables|Internal|GetForwardVector)) (Variables|AutoAimComponent|GetTypesToTrace) false ActorsToIgnore (select (Variables|Debug|GetbDrawTrace) "Persistent" "None") true))
          (bind _output_get_2 (LocalVariables|SetbLocal_HitSuccess _returnvalue))
          (if _output_get_2
            (bind _output_get_3 (Variables|Internal|SetHitLocation (.Location (Collision|BreakHitResult _outhit))))
            (Variables|Internal|SetHitTarget (.HitActor (Collision|BreakHitResult _outhit)))
            (Utilities|FlowControl|Sequence
              (:then_0
                (if (Private|InternalHasLineOfSight)
                  (Default|CallOnAutoAimStarted _outhit)
                  (else
                    (LocalVariables|SetbLocal_HitSuccess false)
                    (Private|InternalTraceFailed "No line of sight to target."))))
              (:then_1
                (if (Variables|Debug|GetbDrawTraceHitSphere)
                  (Rendering|Debug|DrawDebugSphere _output_get_3 4e+01 12 "(R=1.000000,G=0.000000,B=0.000000,A=1.000000)" 8.64e+04))))
            (else
              (Private|InternalTraceFailed "No Trace Hit found."))))))
    (:then_1
      (return (LocalVariables|GetbLocal_HitSuccess)))))

(fn SetActorstoIgnore
  (params (IgnoreActors :type Array%20of%20Actor%20Object%20References))
  (Utilities|Array|Clear (Variables|Internal|GetIgnoreActors))
  (Variables|Internal|SetIgnoreActors IgnoreActors))

(fn IsAimingNow
  (return (Variables|Internal|GetbIsTracingActive)))

(fn InternalTraceFailed
  (params (ErrorMessage :type String))
  (Variables|Internal|SetbIsTracingActive false)
  (Variables|Internal|SetHitTarget 0)
  (Default|CallOnAutoAimFailed ErrorMessage)
  (Development|PrintString ErrorMessage (Variables|Debug|GetbPrintDebugMessages) true "(R=1.000000,G=0.000000,B=0.000000,A=1.000000)" 3e+01))

(fn InternalShowDebugTraceLine
  (if (Variables|Debug|GetbShowDebugTraceLine)
    (Rendering|Debug|FlushPersistentDebugLines)
    (Rendering|Debug|DrawDebugLine (Private|InternalGetLookatStartLocation) (Private|InternalGetLookatTargetLocation) "(R=1.000000,G=0.000000,B=0.008842,A=1.000000)" (Utilities|Time|GetWorldDeltaSeconds) 1.0)))

(fn SetLookatStartLocation
  (params (InStartLocation :type Vector%20%28by%20ref%29))
  (Variables|Internal|SetStartLocation InStartLocation))

(fn SetLookatTargetLocation
  (params (InEndLocation :type Vector%20%28by%20ref%29))
  (Variables|Internal|SetTargetLocation InEndLocation))

(fn InternalGetLookatRotation
  (return (Math|Rotator|FindLookatRotation (Private|InternalGetLookatStartLocation) (Private|InternalGetLookatTargetLocation))))

(fn InternalGetLookatTargetLocation
  (return (select (Variables|AutoAimComponent|GetbUpdateEveryFrame) (select (Variables|Internal|GetbUseManualTargetLocation) (Variables|Internal|GetTargetLocation) (Transformation|GetActorLocation (Variables|Internal|GetHitTarget))) (Variables|Internal|GetHitLocation))))

(fn InternalGetLookatStartLocation
  (return (select (Variables|Internal|GetbUseManualStartLocation) (Variables|Internal|GetStartLocation) (Transformation|GetWorldLocation (Variables|Default|GetStartLookAtComponent)))))

(fn GetHitTarget
  (bind _hittarget (Variables|Internal|GetHitTarget))
  (return (Utilities|IsValid _hittarget) _hittarget))

(fn InternalHasLineOfSight
  (bind (_breturnvalue _outhittarget) (AutoAimComponent|GetHitTarget))
  (bind _ownerpawn (Variables|Internal|GetOwnerPawn))
  (LocalVariables|SetbLocal_HasLineOfSight true)
  (Utilities|FlowControl|Sequence
    (:then_0
      (if (Variables|AutoAimComponent|GetbCheckLineOfSight)
        (Utilities|IsValid _ownerpawn
          (:Is%20Valid
            (if _breturnvalue
              (LocalVariables|SetbLocal_HasLineOfSight (Controller|LineOfSightTo (Pawn|GetController _ownerpawn) _outhittarget "0, 0, 0" false))))
          (:Is%20Not%20Valid
            (Private|InternalTraceFailed "Line of sight check failed. No Owner Pawn set!")))))
    (:then_1
      (return (LocalVariables|GetbLocal_HasLineOfSight)))))