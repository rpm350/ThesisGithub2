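; BP_Cannon is a possessable cannon that the player loads by rolling a BP_Cannonball into it, then aims and fires.
; On overlap it blends the camera, possesses itself after a delay, resets highlight and selection state, and destroys the ball.
; Once loaded, Perform plays a sound and spawns a FirstPersonProjectile from the Spawner along the follow camera's rotation.
; Turn and LookUp drive controller yaw and pitch, overriding the ball template's mouse input.
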(event EventBeginPlay)

(event Collision|EventActorBeginOverlap
  (params (OtherActor :type Actor%20Object%20Reference))
  (bind _returnvalue (Game|Player|GetPlayerPawn 0))
  (bind _returnvalue_2 (Game|GetPlayerController 0))
  (bind _staticmesh (Variables|Default|GetStaticMesh))
  ;[1 1 1] Load Cannon by rolling the ball
  (bind _asbp_cannonball (Utilities|Casting|CastToBP_Cannonball OtherActor)
    (:then
      (Variables|Default|Setloaded true)
      ;[1 1 1] Possess/Transfer
      (Rendering|Material|SetMaterial (Variables|/Game/Interactables/PossesedObjects/BallTemplate.BallTemplate_C|GetStaticMesh _asbp_cannonball) 0 (Variables|/Game/Interactables/PossesedObjects/BallTemplate.BallTemplate_C|GetmydefaultMaterial _asbp_cannonball))
      (Components|Movement|StopMovementImmediately (Variables|Character|GetCharacterMovement))
      (CallFunction|UnHighlight)
      (Input|DisableInput _returnvalue _returnvalue_2)
      ;[1 1 1] Camera Transition to Possess
      (Game|Player|SetViewTargetwithBlend (Game|GetPlayerController 0) 0 1.5 "VTBlend_Cubic" 0.0 false)
      (Utilities|FlowControl|Delay 2.0)
      (Pawn|Possess _returnvalue_2 self)
      (Input|EnableInput _returnvalue _returnvalue_2)
      (Rendering|Material|SetMaterial _staticmesh 0 (Variables|Default|GetmydefaultMaterial))
      (Rendering|SetRenderCustomDepth _staticmesh false)
      (Variables|Default|SetselectedPawn 0)
      (Actor|DestroyActor OtherActor))
    (:CastFailed
      (Development|PrintString "Hello"))))

(event EventTick
  (params (DeltaSeconds :type Float%20%28single-precision%29))
  (|CallParentFunction DeltaSeconds) ; This node is disabled and will not be called.\nDrag off pins to build functionality.
)

(event Input|ActionEvents|InputActionPerform
  (params (Key :type Key%20Structure))
  (bind _followcamera (Variables|Default|GetFollowCamera))
  (bind _returnvalue (Transformation|GetWorldRotation _followcamera))
  (:Pressed
    (if (Variables|Default|Getloaded)
      (Audio|Components|Audio|Play (Variables|Default|GetcannonFire_sound) 0.0)
      (Game|SpawnActorfromClass "/Game/FirstPersonBP/Blueprints/FirstPersonProjectile.FirstPersonProjectile_C" (Math|Transform|MakeTransform (+ (Transformation|GetWorldLocation (Variables|Default|Getspawner)) (Math|Vector|RotateVector (Variables|Default|GetcannonOffset) _returnvalue)) _returnvalue) "Undefined" 0 0))))

(event Input|AxisEvents|InputAxisLookUp
  (params (AxisValue :type Float%20%28single-precision%29))
  ;[1 1 1] Mouse input- Overriding Ball Template
  (Pawn|Input|AddControllerPitchInput AxisValue))

(event Input|AxisEvents|InputAxisTurn
  (params (AxisValue :type Float%20%28single-precision%29))
  ;[1 1 1] Mouse input- Overriding Ball Template
  (Pawn|Input|AddControllerYawInput AxisValue))

(fn ConstructionScript
  (|CallParentFunction))