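; BP_CongaDrum01 is an interactable conga drum that plays a sound when the Perform input action is pressed.
; Pressing Perform starts the Sound from the beginning and sets a Playing flag.
; Tick clears that flag once the sound stops playing.
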(event EventBeginPlay
  (|CallParentFunction) ; This node is disabled and will not be called.\nDrag off pins to build functionality.
)

(event Collision|EventActorBeginOverlap
  (params (OtherActor :type Actor%20Object%20Reference)))

(event EventTick
  (params (DeltaSeconds :type Float%20%28single-precision%29))
  (|CallParentFunction DeltaSeconds)
  (if (Variables|Default|Getplaying)
    (if (not (Audio|Components|Audio|IsPlaying (Variables|Default|Getsound)))
      (Variables|Default|Setplaying false))))

(event Input|ActionEvents|InputActionPerform
  (params (Key :type Key%20Structure))
  (:Pressed
    (Audio|Components|Audio|Play (Variables|Default|Getsound) 0.0)
    (Variables|Default|Setplaying true)))

(fn ConstructionScript
  (|CallParentFunction))