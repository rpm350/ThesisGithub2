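; Interactable sound board sliders that, on the Perform input, set off a one-shot speaker feedback and glass-breaking event.
; Pressing slides the mesh toward Start with camera shake, then staggered delays play feedback and breaking-glass audio, damage a destructible and enable physics on a falling object.
; Done blocks repeats once valid glass is damaged.
; Releasing always slides the mesh toward Finish after a delay.
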(event EventBeginPlay
  (|CallParentFunction) ; This node is disabled and will not be called.\nDrag off pins to build functionality.
)

(event Collision|EventActorBeginOverlap
  (params (OtherActor :type Actor%20Object%20Reference)))

(event Input|ActionEvents|InputActionPerform
  (params (Key :type Key%20Structure))
  (bind _glassbreak (Variables|Default|GetGlassBreak))
  (bind _rootcomponent (Variables|/Script/Engine.Actor|GetRootComponent _glassbreak))
  (bind _returnvalue (Transformation|GetWorldLocation _rootcomponent))
  (:Pressed
    (if (not (Variables|Default|Getdone))
      (Utilities|FlowControl|Sequence
        (:then_0
          (bind _newtrack_0 (Timeline|Timeline_0 Play)
            (:Update
              (Transformation|SetRelativeLocation (Variables|Default|GetStaticMesh) (Math|Vector|Lerp(Vector) (.Location (Math|Transform|BreakTransform (Transformation|GetRelativeTransform (Variables|Default|GetStaticMesh)))) (Variables|Default|GetStart) _newtrack_0) false false)
              (Class|PlayerController|ClientPlayCameraShake (Game|GetPlayerController 0) "/Game/Interactables/PossesedObjects/BP_CameraShake.BP_CameraShake_C" _newtrack_0 "World" "0, 0, 0"))))
        (:then_1
          (Utilities|FlowControl|Delay 2.0)
          (bind _asbp_falling_object (Utilities|Casting|CastToBP_FallingObject (Variables|Default|GetFallingObject)))
          (Physics|SetSimulatePhysics (Variables|/Game/Interactables/BP_FallingObject.BP_FallingObject_C|GetStaticMesh _asbp_falling_object) true))
        (:then_2
          (Utilities|FlowControl|Delay 0.2)
          (Audio|Components|Audio|Play (Variables|Default|GetSpeakerFeedback) 0.0))
        (:then_3
          (Utilities|FlowControl|Delay 1.0)
          (Audio|Components|Audio|Play (Variables|Default|GetBreakingGlass) 0.0)
          (Utilities|IsValid _glassbreak
            (:Is%20Valid
              (Class|DestructibleComponent|ApplyDamage (Variables|/Script/ApexDestruction.DestructibleActor|GetDestructibleComponent _glassbreak) 1.0 _returnvalue _returnvalue 2.0)
              (Variables|Default|Setdone true)
              (Variables|Default|SetshowButtonPressed true)))))))
  (:Released
    (Utilities|FlowControl|Delay 5.0)
    (bind _newtrack_0_2 (Timeline|Timeline_2 Play)
      (:Update
        (Transformation|SetRelativeLocation (Variables|Default|GetStaticMesh) (Math|Vector|Lerp(Vector) (.Location (Math|Transform|BreakTransform (Transformation|GetRelativeTransform (Variables|Default|GetStaticMesh)))) (Variables|Default|GetFinish) _newtrack_0_2) false false)))))

(fn ConstructionScript
  (|CallParentFunction))