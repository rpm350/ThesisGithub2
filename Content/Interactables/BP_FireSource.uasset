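; BP_FireSource is an interactable fire that the Perform input toggles on and off, igniting nearby puddles.
; Overlapping BP_Puddle actors copy the source's fire state and effect, but are only stored in an array when the source is unlit.
; Lighting it plays a sound and ignites stored puddles via SetOnFire, which the overlap path skips.
; Extinguishing affects only the source, and the array is never pruned.
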(event EventBeginPlay)

(event Collision|EventActorBeginOverlap
  (params (OtherActor :type Actor%20Object%20Reference))
  (bind _asbp_puddle (Utilities|Casting|CastToBP_Puddle OtherActor))
  (if (Variables|Default|GetonFire)
    (Variables|/Game/Interactables/BP_Puddle.BP_Puddle_C|SetonFire _asbp_puddle true)
    (Components|Activation|Activate (Variables|/Game/Interactables/BP_Puddle.BP_Puddle_C|Getfire _asbp_puddle) false)
    (else
      (Variables|/Game/Interactables/BP_Puddle.BP_Puddle_C|SetonFire _asbp_puddle false)
      (Components|Activation|Deactivate (Variables|/Game/Interactables/BP_Puddle.BP_Puddle_C|Getfire _asbp_puddle))
      (Utilities|Array|Add (Variables|Default|GettouhcingPuddles) _asbp_puddle))))

(event EventTick
  (params (DeltaSeconds :type Float%20%28single-precision%29))
  (|CallParentFunction DeltaSeconds) ; This node is disabled and will not be called.\nDrag off pins to build functionality.
)

(event Input|ActionEvents|InputActionPerform
  (params (Key :type Key%20Structure))
  (:Pressed
    (if (Variables|Default|GetonFire)
      (Variables|Default|SetonFire false)
      (Components|Activation|Deactivate (Variables|Default|Getfire))
      (else
        (Audio|Components|Audio|Play (Variables|Default|Getfire_sound) 0.0)
        (Variables|Default|SetonFire true)
        (Components|Activation|Activate (Variables|Default|Getfire) false)
        (for _array_element (Variables|Default|GettouhcingPuddles)
          (Development|PrintString "fire")
          (Variables|/Game/Interactables/BP_Puddle.BP_Puddle_C|SetonFire _array_element true)
          (Components|Activation|Activate (Variables|/Game/Interactables/BP_Puddle.BP_Puddle_C|Getfire _array_element) false)
          (Default|SetonFire _array_element))))))

(fn ConstructionScript
  (|CallParentFunction))