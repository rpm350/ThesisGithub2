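; BP_GasCan is an interactable gas can that emits a timed burst of gas when the Perform input action is pressed.
; The press activates the particle system, starts the Gas sound and sets a GasOn flag.
; While flagged, Tick replays the sound whenever it ends, printing the timer for debugging.
; A frame-counted, frame-rate-dependent timer then clears the flag and deactivates the particles, without explicitly stopping the sound.
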(event EventBeginPlay
  (|CallParentFunction) ; This node is disabled and will not be called.\nDrag off pins to build functionality.
)

(event Collision|EventActorBeginOverlap
  (params (OtherActor :type Actor%20Object%20Reference)))

(event EventTick
  (params (DeltaSeconds :type Float%20%28single-precision%29))
  (bind _gas (Variables|Default|Getgas))
  (|CallParentFunction DeltaSeconds)
  (if (Variables|Default|GetgasOn)
    (if (Audio|Components|Audio|IsPlaying _gas)
      _
      (else
        (Audio|Components|Audio|Play _gas 0.0)
        (Development|PrintString (Utilities|String|ToString(Integer) (Variables|Default|GetgasTimer)))))
    (bind _output_get (Variables|Default|SetgasTimer (+ (Variables|Default|GetgasTimer) 1)))
    (if (>= _output_get 300)
      (Variables|Default|SetgasOn false)
      (Variables|Default|SetgasTimer 0)
      (Components|Activation|Deactivate (Variables|Default|GetParticleSystem)))))

(event Input|ActionEvents|InputActionPerform
  (params (Key :type Key%20Structure))
  (:Pressed
    (Components|Activation|Activate (Variables|Default|GetParticleSystem) false)
    (Variables|Default|SetgasOn true)
    (Audio|Components|Audio|Play (Variables|Default|Getgas) 0.0)))

(fn ConstructionScript
  (|CallParentFunction))