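; BP_StageDoors is a pair of double stage doors that swing open on openDoor and then close themselves.
; openDoor plays an opening sound and sets the Open flag, and Tick interpolates both pivot components in opposite directions with RInterpTo.
; When door B reaches its open world rotation, the state flips to Close, easing both back to zero and playing the closing sound once done.
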(event Custom|openDoor
  (Variables|Default|Setopen true)
  (Audio|PlaySoundatLocation "/Game/Audio/RXN/StagePuzzleRXN/doorOpen.doorOpen" (Transformation|GetActorLocation) "0, 0, 0" 1.0 1.0 0.0 "/Game/Audio/Attn/AISpeaking.AISpeaking" 0 0))

(event EventBeginPlay)

(event Collision|EventActorBeginOverlap
  (params (OtherActor :type Actor%20Object%20Reference)))

(event EventTick
  (params (DeltaSeconds :type Float%20%28single-precision%29))
  (bind _doorbrotpoint (Variables|Default|GetdoorBRotPoint))
  (bind _doorbrotpoint_2 (Variables|Default|GetdoorBRotPoint))
  (bind _doorarotpoint (Variables|Default|GetdoorARotPoint))
  (bind _doorarotpoint_2 (Variables|Default|GetdoorARotPoint))
  (if (Variables|Default|Getopen)
    ;[1 1 1] Rotate B door
    (Transformation|SetWorldRotation _doorbrotpoint_2 (Math|Interpolation|RInterpTo (Transformation|GetWorldRotation _doorbrotpoint_2) "0,-120.000000, 0" DeltaSeconds 5.0) false false)
    ;[1 1 1] Rotate A door
    (Transformation|SetWorldRotation _doorarotpoint (Math|Interpolation|RInterpTo (Transformation|GetWorldRotation _doorarotpoint) "0,120.000000, 0" DeltaSeconds 5.0) false false)
    ;[1 1 1] Check if ready to close
    (if (Math|Rotator|Equal(Rotator) (Transformation|GetWorldRotation (Variables|Default|GetdoorBRotPoint)) "0,-120.000000, 0" 0.01)
      (Variables|Default|Setopen false)
      (Variables|Default|Setclose true))
    (elif (Variables|Default|Getclose)
      ;[1 1 1] Close B door
      (Transformation|SetWorldRotation _doorbrotpoint (Math|Interpolation|RInterpTo (Transformation|GetWorldRotation _doorbrotpoint) "0, 0, 0" DeltaSeconds 5.0) false false)
      ;[1 1 1] Close A door
      (Transformation|SetWorldRotation _doorarotpoint_2 (Math|Interpolation|RInterpTo (Transformation|GetWorldRotation _doorarotpoint_2) "0, 0, 0" DeltaSeconds 5.0) false false)
      ;[1 1 1] Check if done closing
      (if (Math|Rotator|Equal(Rotator) (Transformation|GetWorldRotation (Variables|Default|GetdoorBRotPoint)) "0, 0, 0" 0.01)
        (Variables|Default|Setopen false)
        (Variables|Default|Setclose false)
        (Audio|PlaySoundatLocation "/Game/Audio/RXN/StagePuzzleRXN/doorClose.doorClose" (Transformation|GetActorLocation) "0, 0, 0" 1.0 1.0 0.0 "/Game/Audio/Attn/AISpeaking.AISpeaking" 0 0)))))

(fn ConstructionScript)