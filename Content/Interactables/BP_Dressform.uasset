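; BP_Dressform is a movable dressform interactable that feeds the MoveForward axis into movement input along Forward.
; A head-mounted-display check choosing camera or actor forward vector is left unused.
; AbsVal is a threshold test returning true when X or Z differs by at least PuddleDiam.
; It compares zero vectors, ignoring its CurrentPos and PrevPos inputs, and is not called here.
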(event Input|AxisEvents|InputAxisMoveForward
  (params (AxisValue :type Float%20%28single-precision%29))
  ;[1 1 1] movement
  (Pawn|Input|AddMovementInput (Variables|Default|Getforward) AxisValue false))

(fn ConstructionScript
  (|CallParentFunction))

(fn AbsVal
  (params (currentPos :type Vector) (prevPos :type Vector))
  (bind (_x _y _z) (Math|Vector|BreakVector "0, 0, 0"))
  (bind (_x_2 _y_2 _z_2) (Math|Vector|BreakVector "0, 0, 0"))
  (bind _puddlediam (Variables|Default|GetpuddleDiam))
  (Variables|Default|SetabsVal_x false)
  (Variables|Default|SetabsVal_z false)
  (if (< _x (+ _x_2 _puddlediam))
    ;[1 1 1] Change is too small
    (Variables|Default|SetabsVal_x false)
    (if (> _x (- _x_2 _puddlediam))
      (Variables|Default|SetabsVal_x false)
      (if (< _z (+ _z_2 _puddlediam))
        (Variables|Default|SetabsVal_z false)
        (if (> _z (- _z_2 _puddlediam))
          (Variables|Default|SetabsVal_z false)
          (return false)
          (else
            (Variables|Default|SetabsVal_z true)))
        (else
          (Variables|Default|SetabsVal_z true)))
      (return true)
      (else
        (Variables|Default|SetabsVal_x true)))
    (else
      (Variables|Default|SetabsVal_x true)))
  (return true))