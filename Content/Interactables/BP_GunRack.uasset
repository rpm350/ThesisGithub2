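; BP_GunRack is a one-shot interactable gun rack that, on the Perform input, slides to a target position and blocks path A on the stage controller.
; The press activates smoke and gunshot-cart audio, then, if the controller is valid, sets BlockedA and stops the smoke after a short delay.
; Tick eases the actor toward TargetToPushTo with VInterpTo, using a Y-only threshold to end the push.
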(event EventBeginPlay
  (|CallParentFunction) ; This node is disabled and will not be called.\nDrag off pins to build functionality.
)

(event Collision|EventActorBeginOverlap
  (params (OtherActor :type Actor%20Object%20Reference)))

(event EventTick
  (params (DeltaSeconds :type Float%20%28single-precision%29))
  (|CallParentFunction DeltaSeconds)
  (if (Variables|Default|Getpush)
    (Transformation|SetActorLocation (Math|Interpolation|VInterpTo (Transformation|GetActorLocation) (Variables|Default|GettargetToPushTo) DeltaSeconds 1.0) false false)
    (if (>= (- (.Y (Math|Vector|BreakVector (Variables|Default|GettargetToPushTo))) 0.1) (.Y (Math|Vector|BreakVector (Transformation|GetActorLocation))))
      (Variables|Default|Setpush false))))

(event Input|ActionEvents|InputActionPerform
  (params (Key :type Key%20Structure))
  (bind _mystagecontroller (Variables|Default|GetmyStageController))
  (:Pressed
    (if (not (Variables|Default|GethaveShot))
      (Components|Activation|Activate (Variables|Default|GetPFX_GunRackSmoke) false)
      (Audio|Components|Audio|Play (Variables|Default|GetgunShotRollCart) 0.0)
      (Variables|Default|SethaveShot true)
      (Variables|Default|Setpush true)
      (Utilities|IsValid _mystagecontroller
        (:Is%20Valid
          (Variables|/Game/Interactables/BP_StagePuzzleController.BP_StagePuzzleController_C|SetblockedA _mystagecontroller true)
          (Development|PrintString "BLOCKEDA")
          (Utilities|FlowControl|Delay 0.2)
          (Components|Activation|Deactivate (Variables|Default|GetPFX_GunRackSmoke)))))))

(fn ConstructionScript
  (|CallParentFunction))