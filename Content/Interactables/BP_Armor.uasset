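; BP_Armor is an interactable armor actor that swings its Spear component when the Perform input action is pressed.
; The press is accepted only while Ready, playing AxeWhoosh and starting the swing.
; Tick uses RInterpTo on world rotation to move the spear to SwingRotation, then back to BaseRotation, driven by Swing and SwingBack flags.
; Once back, it zeroes the working rotation and re-arms for the next press.
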(event EventBeginPlay
  (|CallParentFunction) ; This node is disabled and will not be called.\nDrag off pins to build functionality.
)

(event Collision|EventActorBeginOverlap
  (params (OtherActor :type Actor%20Object%20Reference)))

(event EventTick
  (params (DeltaSeconds :type Float%20%28single-precision%29))
  (|CallParentFunction DeltaSeconds)
  (if (Variables|Default|Getswing)
    (if (Math|Rotator|Equal(Rotator) (Variables|Default|GetmoveRot) (Variables|Default|GetswingRotation) 0.1)
      (Variables|Default|SetswingBack true)
      (Variables|Default|Setswing false)
      (else
        (bind _output_get (Variables|Default|SetmoveRot (Math|Interpolation|RInterpTo (Variables|Default|GetmoveRot) (Variables|Default|GetswingRotation) DeltaSeconds 1e+01)))
        (Transformation|SetWorldRotation (Variables|Default|Getspear) _output_get false false)))
    (elif (Variables|Default|GetswingBack)
      (if (Math|Rotator|Equal(Rotator) (Variables|Default|GetmoveRot) (Variables|Default|GetbaseRotation) 0.1)
        (Variables|Default|SetswingBack false)
        (Variables|Default|SetmoveRot "0, 0, 0")
        (Variables|Default|Setready true)
        (else
          (bind _output_get_2 (Variables|Default|SetmoveRot (Math|Interpolation|RInterpTo (Variables|Default|GetmoveRot) (Variables|Default|GetbaseRotation) DeltaSeconds 1e+01)))
          (Transformation|SetWorldRotation (Variables|Default|Getspear) _output_get_2 false false))))))

(event Input|ActionEvents|InputActionPerform
  (params (Key :type Key%20Structure))
  (:Pressed
    (if (Variables|Default|Getready)
      (Variables|Default|Setswing true)
      (Variables|Default|Setready false)
      (Audio|Components|Audio|Play (Variables|Default|GetaxeWhoosh) 0.0))))

(fn ConstructionScript
  (|CallParentFunction))