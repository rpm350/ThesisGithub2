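; Stage puzzle controller that runs a fire alarm sequence, sending a Distractable AI through the stage along switchable waypoint routes.
; Perform opens the start doors and spawns the AI with a behavior tree at the start terminal, unless Died or already Running.
; Tick polls blocked flags to replace route A's waypoints with B's, then B's with C's.
; Separate events halt the AI or end the run by opening the end doors and destroying it.
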(event Custom|spawnBPath
  ;[1 1 1] Spawn B Path
  (for (_array_element _array_index) (Variables|Default|GetBPathLocs)
    (bind _returnvalue (Game|SpawnActorfromClass "/Game/Characters/NPC/PatrolAI/AI_DistractableParent/BP_AIWaypoint.BP_AIWaypoint_C" (Math|Conversions|ToTransform(Vector) _array_element) "Undefined" 0 0))
    (Variables|/Game/Characters/NPC/PatrolAI/AI_DistractableParent/BP_AIWaypoint.BP_AIWaypoint_C|SetPosition _returnvalue _array_index)
    (if (== _array_index 0)
      (Variables|Default|SetBpath_0 _returnvalue)
      (elif (== _array_index 1)
        (Variables|Default|SetBpath_1 _returnvalue)
        (elif (== _array_index 2)
          (Variables|Default|SetBpath_2 _returnvalue)
          (elif (== _array_index 3)
            (Variables|Default|SetBpath_3 _returnvalue))))))
  (Variables|Default|SetspawnedBPath true))

(event Custom|endRun
  (bind _myai (Variables|Default|GetmyAI))
  ;[1 1 1] End a run - destroy the AI
  (Default|OpenDoor (Variables|Default|GetmyEndDoors))
  (Variables|Default|Setrunning false)
  (Utilities|IsValid _myai
    (:Is%20Valid
      (Actor|DestroyActor _myai))))

(event Custom|Perform
  ;[1 1 1] Pull the fire alarm
  (if (not (Variables|Default|Getdied))
    (if (not (Variables|Default|Getrunning))
      (Variables|Default|Setrunning true)
      (Default|OpenDoor (Variables|Default|GetmyStartDoors))
      (bind _returnvalue (AI|SpawnAIFromClass "/Game/Characters/NPC/PatrolAI/AI_DistractableParent/Distractable.Distractable_C" "/Game/Characters/NPC/PatrolAI/AI_DistractableParent/BT_AdvancedAI.BT_AdvancedAI" (Transformation|GetActorLocation (Variables|Default|GetstartTerminal)) "0, 0, 0" false))
      (bind _asdistractable (Utilities|Casting|CastToDistractable _returnvalue))
      (bind _output_get (Variables|Default|SetmyAI _asdistractable))
      (Variables|/Script/Engine.CharacterMovementComponent|SetMaxWalkSpeed (Variables|/Script/Engine.Character|GetCharacterMovement (Variables|Default|GetmyAI)) 5e+02)
      (Audio|PlaySoundatLocation "/Game/Audio/RXN/StagePuzzleRXN/RXN_FireAh.RXN_FireAh" (Transformation|GetActorLocation _output_get) "0, 0, 0" 1.0 1.0 0.0 "/Game/Audio/Attn/AISpeaking.AISpeaking" 0 0))))

(event Custom|deleteBPath
  (bind _bpath_0 (Variables|Default|GetBpath_0))
  (bind _bpath_1 (Variables|Default|GetBpath_1))
  (bind _bpath_2 (Variables|Default|GetBpath_2))
  (bind _bpath_3 (Variables|Default|GetBpath_3))
  ;[1 1 1] Delete B Path
  (Utilities|IsValid _bpath_0
    (:Is%20Valid
      (Actor|DestroyActor _bpath_0))
    (:Is%20Not%20Valid
      _))
  (Utilities|IsValid _bpath_1
    (:Is%20Valid
      (Actor|DestroyActor _bpath_1))
    (:Is%20Not%20Valid
      _))
  (Utilities|IsValid _bpath_2
    (:Is%20Valid
      (Actor|DestroyActor _bpath_2))
    (:Is%20Not%20Valid
      _))
  (Utilities|IsValid _bpath_3
    (:Is%20Valid
      (Actor|DestroyActor _bpath_3))))

(event Custom|deleteAPath
  (bind _apath_0 (Variables|Default|GetApath_0))
  (bind _apath_1 (Variables|Default|GetApath_1))
  (bind _apath_2 (Variables|Default|GetApath_2))
  (bind _apath_3 (Variables|Default|GetApath_3))
  ;[1 1 1] Delete A Path
  (Utilities|IsValid _apath_0
    (:Is%20Valid
      (Actor|DestroyActor _apath_0))
    (:Is%20Not%20Valid
      _))
  (Utilities|IsValid _apath_1
    (:Is%20Valid
      (Actor|DestroyActor _apath_1))
    (:Is%20Not%20Valid
      _))
  (Utilities|IsValid _apath_2
    (:Is%20Valid
      (Actor|DestroyActor _apath_2))
    (:Is%20Not%20Valid
      _))
  (Utilities|IsValid _apath_3
    (:Is%20Valid
      (Actor|DestroyActor _apath_3))))

(event Custom|stopMoving
  (bind _myai (Variables|Default|GetmyAI))
  ;[1 1 1] Stop moving the AI - set walking speed to 0
  (Utilities|IsValid _myai
    (:Is%20Valid
      (Variables|/Script/Engine.CharacterMovementComponent|SetMaxWalkSpeed (Variables|/Script/Engine.Character|GetCharacterMovement _myai) 0.0))))

(event Custom|respawnCurrentPath
  ;[1 1 1] Respawn Current Path
)

(event Custom|spawnAPath
  ;[1 1 1] Spawn A path
  (for (_array_element _array_index) (Variables|Default|GetAPathLocs)
    (bind _returnvalue (Game|SpawnActorfromClass "/Game/Characters/NPC/PatrolAI/AI_DistractableParent/BP_AIWaypoint.BP_AIWaypoint_C" (Math|Conversions|ToTransform(Vector) _array_element) "Undefined" 0 0))
    (Variables|/Game/Characters/NPC/PatrolAI/AI_DistractableParent/BP_AIWaypoint.BP_AIWaypoint_C|SetPosition _returnvalue _array_index)
    (if (== _array_index 0)
      (Variables|Default|SetApath_0 _returnvalue)
      (elif (== _array_index 1)
        (Variables|Default|SetApath_1 _returnvalue)
        (elif (== _array_index 2)
          (Variables|Default|SetApath_2 _returnvalue)
          (elif (== _array_index 3)
            (Variables|Default|SetApath_3 _returnvalue)))))))

(event Custom|spawnCPath
  ;[1 1 1] Spawn C path
  (for (_array_element _array_index) (Variables|Default|GetCPathLocs)
    (bind _returnvalue (Game|SpawnActorfromClass "/Game/Characters/NPC/PatrolAI/AI_DistractableParent/BP_AIWaypoint.BP_AIWaypoint_C" (Math|Conversions|ToTransform(Vector) _array_element) "Undefined" 0 0))
    (Variables|/Game/Characters/NPC/PatrolAI/AI_DistractableParent/BP_AIWaypoint.BP_AIWaypoint_C|SetPosition _returnvalue _array_index)
    (if (== _array_index 0)
      (Variables|Default|SetCpath_0 _returnvalue)))
  (Variables|Default|SetcPathSpawned true))

(event EventBeginPlay)

(event Collision|EventActorBeginOverlap
  (params (OtherActor :type Actor%20Object%20Reference)))

(event EventTick
  (params (DeltaSeconds :type Float%20%28single-precision%29))
  (if (Variables|Default|GetblockedA)
    (if (Variables|Default|GetApathGone)
      (if (Variables|Default|GetblockedB)
        (if (not (Variables|Default|GetBpathGone))
          (CallFunction|DeleteBPath)
          (Variables|Default|SetBpathGone true)
          (CallFunction|SpawnCPath)))
      (else
        (CallFunction|DeleteAPath)
        (Variables|Default|SetApathGone true)
        (CallFunction|SpawnBPath)))))

(fn ConstructionScript)

(fn SetActorDisabled
  (params (actor :type Actor%20Object%20Reference))
  (Rendering|SetActorHiddenInGame actor true)
  (Collision|SetActorEnableCollision actor false)
  (Actor|Tick|SetActorTickEnabled actor)
  (return))

(fn SetActorEnabled
  (params (actor :type Actor%20Object%20Reference))
  (Rendering|SetActorHiddenInGame actor false)
  (Collision|SetActorEnableCollision true)
  (Actor|Tick|SetActorTickEnabled true)
  (return))