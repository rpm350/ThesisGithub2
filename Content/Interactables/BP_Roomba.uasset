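; Roomba actor that the Perform input toggles on and off with its sound, travelling a looping route of points while on.
; Overlapping a BP_RoombaPoint advances the index through MyPoints and sets a look-at target rotation.
; Tick lerps location toward the current point and eases rotation toward that target.
; Mouse input turns the controller and reapplies the stored mesh rotation, overriding the Ball Template's movement.
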(event EventBeginPlay
  ;[1 1 1] Give roomba a sitting still rotation
  (Variables|Default|SetmoveRot (Transformation|GetWorldRotation (Variables|Default|GetStaticMesh))))

(event Collision|EventActorBeginOverlap
  (params (OtherActor :type Actor%20Object%20Reference))
  ;[1 1 1] Change direction when you reach a point
  (Utilities|Casting|CastToBP_RoombaPoint OtherActor)
  (Development|PrintString (Utilities|String|ToString(Integer) (Variables|Default|GetcurrentPoint)))
  (if (>= (Variables|Default|GetcurrentPoint) (- (Utilities|Array|Length (Variables|Default|GetmyPoints)) 1))
    (Variables|Default|SetcurrentPoint 0)
    (else
      (Variables|Default|SetcurrentPoint (+ (Variables|Default|GetcurrentPoint) 1))))
  (Variables|Default|SettargetRot (Math|Rotator|FindLookatRotation (Transformation|GetActorLocation) (Transformation|GetActorLocation (Utilities|Array|Get(acopy) (Variables|Default|GetmyPoints) (Variables|Default|GetcurrentPoint)))))
  (Variables|Default|Setmoving true))

(event EventTick
  (params (DeltaSeconds :type Float%20%28single-precision%29))
  (bind _roomba_sound (Variables|Default|Getroomba_sound))
  (|CallParentFunction DeltaSeconds)
  ;[1 1 1] If on, move to next point
  (if (Variables|Default|Geton)
    (if (Audio|Components|Audio|IsPlaying _roomba_sound)
      _
      (else
        (Audio|Components|Audio|Play _roomba_sound 0.0)))
    (Transformation|SetActorLocation (Math|Vector|Lerp(Vector) (Transformation|GetActorLocation) (Transformation|GetActorLocation (Utilities|Array|Get(acopy) (Variables|Default|GetmyPoints) (Variables|Default|GetcurrentPoint))) (* DeltaSeconds (Variables|Default|GetroombaSpeed))) false false)
    (if (Variables|Default|Getmoving)
      ;[1 1 1] Rotate to face next point
      (bind _output_get (Variables|Default|SetmoveRot (Math|Interpolation|RInterpTo (Variables|Default|GetmoveRot) (Variables|Default|GettargetRot) DeltaSeconds 2.0)))
      (Transformation|SetActorRotation _output_get))))

(event Input|ActionEvents|InputActionPerform
  (params (Key :type Key%20Structure))
  ;[1 1 1] PERFORM ACTION - Turn roomba on or off
  (:Pressed
    (if (Variables|Default|Geton)
      (Variables|Default|Seton false)
      (Audio|Components|Audio|Stop (Variables|Default|Getroomba_sound))
      (else
        (Variables|Default|Seton true)
        (Audio|Components|Audio|Play (Variables|Default|Getroomba_sound) 0.0)))))

(event Input|AxisEvents|InputAxisLookUp
  (params (AxisValue :type Float%20%28single-precision%29))
  ;[1 1 1] Mouse input - overriding Ball Template's movement
  (Pawn|Input|AddControllerPitchInput AxisValue)
  (Transformation|SetWorldRotation (Variables|Default|GetStaticMesh) (Variables|Default|GetmoveRot) false false))

(event Input|AxisEvents|InputAxisTurn
  (params (AxisValue :type Float%20%28single-precision%29))
  ;[1 1 1] Mouse input - overriding Ball Template's movement
  (Pawn|Input|AddControllerYawInput AxisValue)
  (Transformation|SetWorldRotation (Variables|Default|GetStaticMesh) (Variables|Default|GetmoveRot) false false))

(fn ConstructionScript
  (|CallParentFunction))