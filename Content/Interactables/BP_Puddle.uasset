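; BP_Puddle is a flammable puddle actor that catches fire from BP_FireSource and spreads it to other puddles.
; Overlaps ignite or extinguish it by the source's state, and either light another puddle or record it in TouchingPuddles.
; SetOnFire recursively spreads fire through those recorded neighbors.
; Tick-counted timers expire unlit puddles and burn out lit ones, destroying all but source puddles, which only stop burning.
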(event Custom|setOnFire
  ;[1 1 1] Set on fire
  (if (Variables|Default|GetonFire)
    (for _array_element (Variables|Default|GettouchingPuddles)
      (Utilities|IsValid _array_element
        (:Is%20Valid
          (if (not (Variables|BP_Puddle_C|GetonFire _array_element))
            (Variables|BP_Puddle_C|SetonFire _array_element true)
            (Development|PrintString "OREO")
            (Components|Activation|Activate (Variables|BP_Puddle_C|Getfire _array_element) false)
            (CallFunction|SetonFire _array_element)))))))

(event EventBeginPlay)

(event Collision|EventActorBeginOverlap
  (params (OtherActor :type Actor%20Object%20Reference))
  (bind _asbp_fire_source (Utilities|Casting|CastToBP_FireSource OtherActor)
    (:then
      (if (Variables|/Game/Interactables/BP_FireSource.BP_FireSource_C|GetonFire _asbp_fire_source)
        (Variables|Default|SetonFire true)
        (Components|Activation|Activate (Variables|Default|Getfire) false)
        (Development|PrintString "transferring fire")
        (for _array_element (Variables|Default|GettouchingPuddles)
          (Variables|BP_Puddle_C|SetonFire _array_element true)
          (Components|Activation|Activate (Variables|BP_Puddle_C|Getfire _array_element) false))
        (else
          (Variables|Default|SetonFire false)
          (Components|Activation|Deactivate (Variables|Default|Getfire)))))
    (:CastFailed
      (bind _asbp_puddle (Utilities|Casting|CastToBP_Puddle OtherActor))
      (if (Variables|Default|GetonFire)
        (Variables|BP_Puddle_C|SetonFire _asbp_puddle true)
        (Components|Activation|Activate (Variables|BP_Puddle_C|Getfire _asbp_puddle) false)
        (else
          (Utilities|Array|Add (Variables|Default|GettouchingPuddles) _asbp_puddle))))))

(event EventTick
  (params (DeltaSeconds :type Float%20%28single-precision%29))
  (if (Variables|Default|GetsourcePuddle)
    _
    (elif (Variables|Default|GetonFire)
      _
      (else
        (bind _output_get (Variables|Default|SetlifeTimer (+ (Variables|Default|GetlifeTimer) 1)))
        (if (>= _output_get (Variables|Default|GetlifeSpan))
          (Actor|DestroyActor)))))
  ;[1 1 1] burn off
  (if (Variables|Default|GetonFire)
    (bind _output_get_2 (Variables|Default|SetfireTimer (+ (Variables|Default|GetfireTimer) 1)))
    (if (> _output_get_2 (Variables|Default|GetmaxFireLife))
      (Components|Activation|Deactivate (Variables|Default|Getfire))
      (Utilities|FlowControl|Delay 0.5)
      (if (Variables|Default|GetsourcePuddle)
        (Variables|Default|SetonFire false)
        (else
          (Actor|DestroyActor))))))

(fn ConstructionScript)