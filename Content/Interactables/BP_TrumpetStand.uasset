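; BP_TrumpetStand is an interactable trumpet stand that the player performs on to make noise.
; Pressing Perform shows the pressed button state, plays one of three trumpet sounds via chained random rolls, and triggers its reaction volume.
; It also alerts a living sound hunter not already targeting it, making the stand that hunter's current target.
; The check that would clear the Playing flag when audio stops is disconnected.
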(event Custom|getSound
  (bind _numsounds (Variables|Default|GetnumSounds))
  (bind _returnvalue (Math|Random|RandomInteger _numsounds))
  (if (== _returnvalue 0)
    (Audio|Components|Audio|Play (Variables|Default|Gettrumpet) 0.0)
    (elif (== _returnvalue 1)
      (Audio|Components|Audio|Play (Variables|Default|Gettrumpet2) 0.0)
      (else
        (Audio|Components|Audio|Play (Variables|Default|Gettrumpet3) 0.0)))))

(event EventBeginPlay
  (|CallParentFunction) ; This node is disabled and will not be called.\nDrag off pins to build functionality.
)

(event Collision|EventActorBeginOverlap
  (params (OtherActor :type Actor%20Object%20Reference)))

(event EventTick
  (params (DeltaSeconds :type Float%20%28single-precision%29))
  (|CallParentFunction DeltaSeconds))

(event Input|ActionEvents|InputActionPerform
  (params (Key :type Key%20Structure))
  (bind _self self)
  (bind _mysoundhunter (Variables|Default|GetmySoundHunter))
  (bind _myrxnvolume (Variables|Default|GetmyRxnVolume))
  (:Pressed
    ;[1 1 1] Show the pressed UI button?
    (Variables|Default|SetshowPressedButton true)
    (CallFunction|GetSound)
    (Variables|Default|Setplaying true)
    (Utilities|IsValid _myrxnvolume
      (:Is%20Valid
        (Default|React _myrxnvolume))
      (:Is%20Not%20Valid
        _))
    (Utilities|IsValid _mysoundhunter
      (:Is%20Valid
        (if (not (Variables|/Game/Characters/NPC/PatrolAI/AI_DistractableChild_01/Distractable_Child01.Distractable_Child01_C|Getdead _mysoundhunter))
          (if (!= (Variables|/Game/Characters/NPC/PatrolAI/AI_DistractableChild_01/Distractable_Child01.Distractable_Child01_C|GetcurrentTarget _mysoundhunter) _self)
            (Default|HeardSound _mysoundhunter (Variables|Default|GetmySoundHunterTarget))
            (Variables|/Game/Characters/NPC/PatrolAI/AI_DistractableChild_01/Distractable_Child01.Distractable_Child01_C|SetcurrentTarget _mysoundhunter _self))))))
  (:Released
    (Variables|Default|SetshowPressedButton false)))

(fn ConstructionScript
  (|CallParentFunction))