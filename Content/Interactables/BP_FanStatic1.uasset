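; BP_FanStatic1 is a pawn-based fan interactable with a spinning mesh and its own look controls.
; On BeginPlay it points its RotatingMovement component at StaticMesh1, so only that mesh rotates.
; LookUp and Turn axis inputs drive controller pitch and damped yaw.
; The Turn event also rewrites the player camera manager's yaw limits each time it fires, confining the view to an asymmetric arc.
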(event EventBeginPlay
  (Components|Movement|SetUpdatedComponent (Variables|Default|GetRotatingMovement) (Variables|Default|GetStaticMesh1)))

(event Input|AxisEvents|InputAxisLookUp
  (params (AxisValue :type Float%20%28single-precision%29))
  (Pawn|Input|AddControllerPitchInput AxisValue))

(event Input|AxisEvents|InputAxisTurn
  (params (AxisValue :type Float%20%28single-precision%29))
  (bind _returnvalue (Game|GetPlayerCameraManager 0))
  (Variables|/Script/Engine.PlayerCameraManager|SetViewYawMin _returnvalue -2e+01)
  (Variables|/Script/Engine.PlayerCameraManager|SetViewYawMax _returnvalue 9e+01)
  (Pawn|Input|AddControllerYawInput (* AxisValue 0.35)))

(fn ConstructionScript
  (|CallParentFunction))