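; A swinging door actor that opens while the third-person player character overlaps it and closes when the character leaves.
; Overlap begin and end events only toggle an open flag.
; Tick eases the Bottom component's relative rotation toward the open or closed rotation by lerping from its current value with a frame-time-scaled alpha, giving a decelerating swing without a timeline.
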(event Collision|EventActorBeginOverlap
  (params (OtherActor :type Actor%20Object%20Reference))
  (Utilities|Casting|CastToThirdPersonCharacter OtherActor)
  (Variables|Default|SetIsDoorOpen true))

(event EventTick
  (params (DeltaSeconds :type Float%20%28single-precision%29))
  (bind _returnvalue (* DeltaSeconds 2.0))
  (if (Variables|Default|GetIsDoorOpen)
    (Transformation|SetRelativeRotation (Variables|Default|GetBottom) (Math|Rotator|Lerp(Rotator) (.Rotation (Math|Transform|BreakTransform (Transformation|GetRelativeTransform (Variables|Default|GetBottom)))) (Variables|Default|GetDoorOpenPosition) _returnvalue) false false)
    (else
      (Transformation|SetRelativeRotation (Variables|Default|GetBottom) (Math|Rotator|Lerp(Rotator) (.Rotation (Math|Transform|BreakTransform (Transformation|GetRelativeTransform (Variables|Default|GetBottom)))) (Variables|Default|GetDoorClosedPosition) _returnvalue) false false))))

(event Collision|EventActorEndOverlap
  (params (OtherActor :type Actor%20Object%20Reference))
  (Utilities|Casting|CastToThirdPersonCharacter OtherActor)
  (Variables|Default|SetIsDoorOpen false))

(fn ConstructionScript)