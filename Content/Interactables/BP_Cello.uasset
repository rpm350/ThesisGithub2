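; BP_Cello is an interactable cello that plays one of three sounds when the Perform input is pressed.
; GetSound picks the clip through nested RandomInteger checks that re-roll, so odds can be uneven.
; Performing sets Playing and, if valid, triggers the reaction volume's React, then notifies a sound hunter via HeardSound.
; Tick clears Playing once the Audio component stops playing.
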(event Custom|getSound
  (bind _numsounds (Variables|Default|GetnumSounds))
  (bind _returnvalue (Math|Random|RandomInteger _numsounds))
  (if (== _returnvalue 0)
    (Audio|Components|Audio|Play (Variables|Default|Getcello1) 0.0)
    (elif (== _returnvalue 1)
      (Audio|Components|Audio|Play (Variables|Default|Getcello2) 0.0)
      (else
        (Audio|Components|Audio|Play (Variables|Default|Getcello3) 0.0)))))

(event EventBeginPlay
  (|CallParentFunction) ; This node is disabled and will not be called.\nDrag off pins to build functionality.
)

(event Collision|EventActorBeginOverlap
  (params (OtherActor :type Actor%20Object%20Reference)))

(event EventTick
  (params (DeltaSeconds :type Float%20%28single-precision%29))
  (|CallParentFunction DeltaSeconds)
  (if (Variables|Default|Getplaying)
    (if (not (Audio|Components|Audio|IsPlaying (Variables|Default|GetAudio)))
      (Variables|Default|Setplaying false))))

(event Input|ActionEvents|InputActionPerform
  (params (Key :type Key%20Structure))
  (bind _mysoundhunter (Variables|Default|GetmySoundHunter))
  (bind _myrxnvolume (Variables|Default|GetmyRxnVolume))
  (:Pressed
    (CallFunction|GetSound)
    (Variables|Default|Setplaying true)
    (Utilities|IsValid _myrxnvolume
      (:Is%20Valid
        (Default|React _myrxnvolume)
        (Utilities|IsValid _mysoundhunter
          (:Is%20Valid
            (Default|HeardSound _mysoundhunter (Variables|Default|GetmySoundHunterTarget))))))))

(fn ConstructionScript
  (|CallParentFunction))