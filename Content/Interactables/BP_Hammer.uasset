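; Player-controlled hammer, derived from a ball template, that swings on Perform and destroys its assigned door.
; Perform destroys MyDoortoKill immediately if valid, then starts the swing and plays swing and glass-break sounds regardless.
; Tick uses RInterpTo to rotate the actor to SwingRotation and back to BaseRotation via two state flags.
; Mouse input overrides the template's movement, turning the controller and holding mesh world rotation at MoveRot while idle.
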(event EventBeginPlay)

(event Collision|EventActorBeginOverlap
  (params (OtherActor :type Actor%20Object%20Reference)))

(event EventTick
  (params (DeltaSeconds :type Float%20%28single-precision%29))
  (|CallParentFunction DeltaSeconds)
  (if (Variables|Default|Getswing)
    (if (Math|Rotator|Equal(Rotator) (Variables|Default|GetmoveRot) (Variables|Default|GetswingRotation) 0.1)
      (Variables|Default|SetswingBack true)
      (Variables|Default|Setswing false)
      (else
        (bind _output_get (Variables|Default|SetmoveRot (Math|Interpolation|RInterpTo (Variables|Default|GetmoveRot) (Variables|Default|GetswingRotation) DeltaSeconds 5.0)))
        (Transformation|SetActorRotation _output_get)))
    (elif (Variables|Default|GetswingBack)
      (if (Math|Rotator|Equal(Rotator) (Variables|Default|GetmoveRot) (Variables|Default|GetbaseRotation) 0.1)
        (Variables|Default|SetswingBack false)
        (Variables|Default|SetmoveRot "0,180.000000, 0")
        (else
          (bind _output_get_2 (Variables|Default|SetmoveRot (Math|Interpolation|RInterpTo (Variables|Default|GetmoveRot) (Variables|Default|GetbaseRotation) DeltaSeconds 5.0)))
          (Transformation|SetActorRotation _output_get_2))))))

(event Input|ActionEvents|InputActionPerform
  (params (Key :type Key%20Structure))
  (bind _mydoortokill (Variables|Default|GetmyDoortoKill))
  (:Pressed
    (Utilities|IsValid _mydoortokill
      (:Is%20Valid
        (Actor|DestroyActor _mydoortokill))
      (:Is%20Not%20Valid
        _))
    (Variables|Default|Setswing true)
    (Audio|Components|Audio|Play (Variables|Default|Getswing_Sound) 0.0)
    (Audio|Components|Audio|Play (Variables|Default|GetglassBreak_sound) 0.0)))

(event Input|AxisEvents|InputAxisLookUp
  (params (AxisValue :type Float%20%28single-precision%29))
  ;[1 1 1] Mouse input - overriding Ball Template's movement
  (Pawn|Input|AddControllerPitchInput AxisValue)
  (Transformation|SetWorldRotation (Variables|Default|GetStaticMesh) (Variables|Default|GetmoveRot) false false))

(event Input|AxisEvents|InputAxisTurn
  (params (AxisValue :type Float%20%28single-precision%29))
  ;[1 1 1] Mouse input - overriding Ball Template's movement
  (Pawn|Input|AddControllerYawInput AxisValue)
  (if (not (or (Variables|Default|Getswing) (Variables|Default|GetswingBack)))
    (Transformation|SetWorldRotation (Variables|Default|GetStaticMesh) (Variables|Default|GetmoveRot) false false)))

(fn ConstructionScript
  (|CallParentFunction))