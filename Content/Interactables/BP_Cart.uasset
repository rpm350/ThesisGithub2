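; BP_Cart is a possessable cart that becomes drivable when a BP_Wheel overlaps it or its trigger zone.
; That overlap marks it Loaded, blends the camera over, possesses the cart and destroys the wheel.
; MoveForward input then moves it along its starting forward axis and flags CartRolled, so Tick destroys MyBlocker.
; Cannon firing, wheel audio or animation and NPC reaction logic remain as disconnected leftovers.
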(event OnComponentBeginOverlap(triggerzone)
  (params (OverlappedComponent :type Primitive%20Component%20Object%20Reference) (OtherActor :type Actor%20Object%20Reference) (OtherComp :type Primitive%20Component%20Object%20Reference) (OtherBodyIndex :type Integer) (bFromSweep :type Boolean) (SweepResult :type Hit%20Result%20Structure%20%28by%20ref%29))
  (bind _returnvalue (Game|Player|GetPlayerPawn 0))
  (bind _returnvalue_2 (Game|GetPlayerController 0))
  (bind _staticmesh (Variables|Default|GetStaticMesh))
  ;[1 1 1] Load Cannon by rolling the ball
  (bind _asbp_wheel (Utilities|Casting|CastToBP_Wheel OtherActor))
  (Variables|Default|Setloaded true)
  ;[1 1 1] Possess/Transfer
  (Components|Movement|StopMovementImmediately (Variables|Character|GetCharacterMovement))
  (CallFunction|UnHighlight)
  (Input|DisableInput _returnvalue _returnvalue_2)
  ;[1 1 1] Camera Transition to Possess
  (Game|Player|SetViewTargetwithBlend (Game|GetPlayerController 0) 0 0.25 "VTBlend_Cubic" 0.0 false)
  (Utilities|FlowControl|Delay 0.25)
  (Pawn|Possess _returnvalue_2 self)
  (Input|EnableInput _returnvalue _returnvalue_2)
  (Rendering|Material|SetMaterial _staticmesh 0 (Variables|Default|GetmydefaultMaterial))
  (Rendering|SetRenderCustomDepth _staticmesh false)
  (Variables|Default|SetselectedPawn 0)
  (Actor|DestroyActor (stale Collision|EventActorBeginOverlap OtherActor)))

(event EventTick
  (params (DeltaSeconds :type Float%20%28single-precision%29))
  (bind _myblocker (Variables|Default|GetmyBlocker))
  (|CallParentFunction 0.0)
  (if (Variables|Default|Getloaded)
    (if (Variables|Default|GetcartRolled)
      (Utilities|IsValid _myblocker
        (:Is%20Valid
          (Actor|DestroyActor _myblocker))))))

(event Collision|EventActorBeginOverlap
  (params (OtherActor :type Actor%20Object%20Reference))
  (bind _returnvalue (Game|Player|GetPlayerPawn 0))
  (bind _returnvalue_2 (Game|GetPlayerController 0))
  (bind _staticmesh (Variables|Default|GetStaticMesh))
  ;[1 1 1] Load Cannon by rolling the ball
  (bind _asbp_wheel (Utilities|Casting|CastToBP_Wheel (stale OnComponentBeginOverlap(triggerzone) OtherActor)))
  (Variables|Default|Setloaded true)
  ;[1 1 1] Possess/Transfer
  (Components|Movement|StopMovementImmediately (Variables|Character|GetCharacterMovement))
  (CallFunction|UnHighlight)
  (Input|DisableInput _returnvalue _returnvalue_2)
  ;[1 1 1] Camera Transition to Possess
  (Game|Player|SetViewTargetwithBlend (Game|GetPlayerController 0) 0 0.25 "VTBlend_Cubic" 0.0 false)
  (Utilities|FlowControl|Delay 0.25)
  (Pawn|Possess _returnvalue_2 self)
  (Input|EnableInput _returnvalue _returnvalue_2)
  (Rendering|Material|SetMaterial _staticmesh 0 (Variables|Default|GetmydefaultMaterial))
  (Rendering|SetRenderCustomDepth _staticmesh false)
  (Variables|Default|SetselectedPawn 0)
  (Actor|DestroyActor OtherActor))

(event EventBeginPlay
  (bind _returnvalue (Transformation|GetActorForwardVector))
  (Variables|Default|Setforward _returnvalue)
  (Variables|Default|Setbackward (* _returnvalue "-1.000000,-1.000000,-1.000000")))

(event Input|ActionEvents|InputActionPerform
  (params (Key :type Key%20Structure)))

(event Input|AxisEvents|InputAxisMoveForward
  (params (AxisValue :type Float%20%28single-precision%29))
  ;[1 1 1] R - Movement
  (if (Variables|Default|Getloaded)
    (Pawn|Input|AddMovementInput (Variables|Default|Getforward) AxisValue false)
    (if (Variables|Default|Getloaded)
      ;;[1 1 1] Need to detect when movement stops
      (Variables|Default|SetcartRolled true))))

(fn ConstructionScript
  (|CallParentFunction))