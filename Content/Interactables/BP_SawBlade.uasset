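; Saw blade interactable that, when its cut event fires, travels to a target point and back to its start position.
; Tick drives both legs with VInterpTo, spinning the blade and keeping the saw sound playing outbound, then playing a one-shot saw-off sound on return.
; Once home, it clears its motion flags and resets its linked control's done state, pressed display and material so the cycle can run again.
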(event Custom|cut
  (Variables|Default|Setspin true)
  (Variables|Default|Setmove true)
  (Audio|Components|Audio|Play (Variables|Default|Getsaw) 0.0))

(event EventBeginPlay
  (Variables|Default|SetstartVector (Transformation|GetActorLocation)))

(event Collision|EventActorBeginOverlap
  (params (OtherActor :type Actor%20Object%20Reference)))

(event EventTick
  (params (DeltaSeconds :type Float%20%28single-precision%29))
  (bind _returnvalue (Transformation|GetActorLocation))
  (bind _returnvalue_2 (Transformation|GetActorLocation))
  (bind _saw (Variables|Default|Getsaw))
  (bind _targetmovevector (Variables|Default|GettargetMoveVector))
  (bind _startvector (Variables|Default|GetstartVector))
  (bind _mycontrol (Variables|Default|GetmyControl))
  (if (Variables|Default|Getmove)
    (if (Variables|Default|Getreturn)
      (if (Variables|Default|GetplayedSawOff)
        _
        (else
          (Audio|Components|Audio|Play (Variables|Default|GetsawOff) 0.0)
          (Variables|Default|SetplayedSawOff true)))
      (Transformation|SetActorLocation (Math|Interpolation|VInterpTo _returnvalue _startvector DeltaSeconds 1.0) false false)
      (if (Math|Vector|Equal(Vector) _returnvalue _startvector 0.1)
        (Variables|Default|Setreturn false)
        (Variables|Default|Setmove false)
        (Variables|Default|Setspin false)
        (Variables|/Game/Interactables/BP_SawControl.BP_SawControl_C|Setdone _mycontrol false)
        (Variables|/Game/Interactables/BP_SawControl.BP_SawControl_C|SetshowPressedState _mycontrol false)
        (Rendering|Material|SetMaterial (Variables|/Game/Interactables/PossesedObjects/BallTemplate.BallTemplate_C|GetStaticMesh _mycontrol) 0 "/Engine/EngineMeshes/M_Mat_UnrealTech.M_Mat_UnrealTech")
        (Variables|Default|SetplayedSawOff false))
      (else
        (if (Audio|Components|Audio|IsPlaying _saw)
          _
          (else
            (Audio|Components|Audio|Play _saw 0.0)))
        (Transformation|SetActorLocation (Math|Interpolation|VInterpTo _returnvalue_2 _targetmovevector DeltaSeconds 1.0) false false)
        (if (Math|Vector|Equal(Vector) _returnvalue_2 _targetmovevector 0.1)
          (Variables|Default|Setreturn true))
        (if (Variables|Default|Getspin)
          (Transformation|AddActorLocalRotation (Math|Rotator|MakeRotator 0.0 (* (Variables|Default|GetspinRate) DeltaSeconds) 0.0) false false))))))

(fn ConstructionScript)