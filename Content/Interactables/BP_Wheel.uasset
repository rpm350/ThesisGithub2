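; BP_Wheel is a player-controlled rolling pawn with camera-relative movement on the horizontal plane.
; Move axes add movement input along control yaw and set ShowPressedButton, while look axes drive controller yaw and pitch, with rate-scaled variants.
; Tick fakes rolling by accumulating an angle from horizontal speed and Ratio, then setting the static mesh's world rotation about the axis perpendicular to travel.
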(event Collision|EventActorBeginOverlap
  (params (OtherActor :type Actor%20Object%20Reference)))

(event EventTick
  (params (DeltaSeconds :type Float%20%28single-precision%29))
  (bind _returnvalue (Transformation|GetVelocity))
  (|CallParentFunction DeltaSeconds)
  (Variables|Default|SethorizVelocity (Math|Vector|MakeVector (.x _returnvalue) (.y _returnvalue) 0.0))
  (Variables|Default|SethorizSpeed (Math|Vector|VectorLength (Variables|Default|GethorizVelocity)))
  (Math|Float|CompareFloat (Variables|Default|GethorizSpeed) 0.0
    (:>
      (Variables|Default|SetrotationAmount (+ (Variables|Default|GetrotationAmount) (* (/ (Variables|Default|GethorizSpeed) (* (Math|Trig|GetPI) (Variables|Default|Getratio))) (Utilities|Time|GetWorldDeltaSeconds))))
      (Transformation|SetWorldRotation (Variables|Default|GetStaticMesh) (Math|Vector|RotatorfromAxisandAngle (Math|Vector|GetRightVector (Math|Rotator|MakeRotfromX (Math|Vector|Normalize (Variables|Default|GethorizVelocity)))) (Variables|Default|GetrotationAmount)) false false))))

(event EventBeginPlay)

(event Input|AxisEvents|InputAxisTurn
  (params (AxisValue :type Float%20%28single-precision%29))
  ;[1 1 1] turning
  (Pawn|Input|AddControllerYawInput AxisValue))

(event Input|AxisEvents|InputAxisLookUp
  (params (AxisValue :type Float%20%28single-precision%29))
  ;[1 1 1] turning
  (Pawn|Input|AddControllerPitchInput AxisValue))

(event Input|AxisEvents|InputAxisTurnRate
  (params (AxisValue :type Float%20%28single-precision%29))
  ;[1 1 1] turn
  (Pawn|Input|AddControllerYawInput (* AxisValue (Variables|Default|GetBaseTurnRate) (Utilities|Time|GetWorldDeltaSeconds))))

(event Input|AxisEvents|InputAxisLookUpRate
  (params (AxisValue :type Float%20%28single-precision%29))
  ;[1 1 1] turn
  (Pawn|Input|AddControllerPitchInput (* AxisValue (Variables|Default|GetBaseLookUpRate) (Utilities|Time|GetWorldDeltaSeconds))))

(event Input|AxisEvents|InputAxisMoveForward
  (params (AxisValue :type Float%20%28single-precision%29))
  ;[1 1 1] T - Movement
  (Pawn|Input|AddMovementInput (Math|Vector|GetForwardVector (Math|Rotator|MakeRotator 0.0 0.0 (.Yaw (Math|Rotator|BreakRotator (Pawn|GetControlRotation :!class /Script/Engine.Pawn))))) AxisValue false)
  (if (== AxisValue 0.0)
    (Variables|Default|SetshowPressedButton false)
    (else
      (Variables|Default|SetshowPressedButton true))))

(event Input|AxisEvents|InputAxisMoveRight
  (params (AxisValue :type Float%20%28single-precision%29))
  ;[1 1 1] T - Movement
  (Pawn|Input|AddMovementInput (Math|Vector|GetRightVector (Math|Rotator|MakeRotator 0.0 0.0 (.Yaw (Math|Rotator|BreakRotator (Pawn|GetControlRotation :!class /Script/Engine.Pawn))))) AxisValue false)
  (if (== AxisValue 0.0)
    (Variables|Default|SetshowPressedButton false)
    (else
      (Variables|Default|SetshowPressedButton true))))

(fn ConstructionScript
  (|CallParentFunction))