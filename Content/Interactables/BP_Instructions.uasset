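; BP_Instructions is an interactable actor that shows control instructions matching the player's input device.
; While its Show flag is set, Tick reads UsingController from POTROGameInstance and makes either ControllerText or MouseText visible, hiding the other.
; The graph has no logic to set Show or to hide both texts when it is off.
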(event EventBeginPlay)

(event Collision|EventActorBeginOverlap
  (params (OtherActor :type Actor%20Object%20Reference)))

(event EventTick
  (params (DeltaSeconds :type Float%20%28single-precision%29))
  (bind _mousetext (Variables|Default|GetmouseText))
  (bind _controllertext (Variables|Default|GetcontrollerText))
  (if (Variables|Default|Getshow)
    (bind _aspotrogame_instance (Utilities|Casting|CastToPOTROGameInstance (Game|GetGameInstance)))
    (if (Variables|/Game/POTROGameInstance.POTROGameInstance_C|GetusingController _aspotrogame_instance)
      (Rendering|SetVisibility _controllertext true false)
      (Rendering|SetVisibility _mousetext false false)
      (else
        (Rendering|SetVisibility _mousetext true false)
        (Rendering|SetVisibility _controllertext false false)))))

(fn ConstructionScript)