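; Interactable fire alarm that sets off its linked sprinklers and notifies a stage puzzle controller.
; The Perform input, ignored while already active, calls the controller, plays alarm and sprinkler audio, and activates each sprinkler's Rain.
; Tick restarts the sprinkler noise if it ends, then after a fixed frame count, not seconds, deactivates the rain, stops that noise and re-arms.
; Despite its name, Ready is true while the alarm runs.
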(event EventBeginPlay
  (|CallParentFunction) ; This node is disabled and will not be called.\nDrag off pins to build functionality.
)

(event Collision|EventActorBeginOverlap
  (params (OtherActor :type Actor%20Object%20Reference)))

(event EventTick
  (params (DeltaSeconds :type Float%20%28single-precision%29))
  (bind _sprinklernoise (Variables|Default|GetsprinklerNoise))
  (|CallParentFunction DeltaSeconds)
  (if (Variables|Default|Getready)
    (bind _output_get (Variables|Default|Settimer (+ (Variables|Default|Gettimer) 1)))
    (if (== _output_get 400)
      (Variables|Default|Setready false)
      (Variables|Default|Settimer 0)
      (for _array_element (Variables|Default|GetmySprinklers)
        (Components|Activation|Deactivate (Variables|/Game/ThirdPersonBP/Blueprints/BP_Sprinkler.BP_Sprinkler_C|Getrain _array_element)))
      (Audio|Components|Audio|Stop (Variables|Default|GetsprinklerNoise))
      (elif (not (Audio|Components|Audio|IsPlaying _sprinklernoise))
        (Audio|Components|Audio|Play _sprinklernoise 0.0)))))

(event Input|ActionEvents|InputActionPerform
  (params (Key :type Key%20Structure))
  (:Pressed
    (if (not (Variables|Default|Getready))
      (Variables|Default|Setready true)
      (Default|Perform (Variables|Default|GetmyStagePuzzleController))
      (Audio|Components|Audio|Play (Variables|Default|GetfireAlarm) 0.0)
      (Audio|Components|Audio|Play (Variables|Default|GetsprinklerNoise) 0.0)
      (for _array_element (Variables|Default|GetmySprinklers)
        (Components|Activation|Activate (Variables|/Game/ThirdPersonBP/Blueprints/BP_Sprinkler.BP_Sprinkler_C|Getrain _array_element) false)))))

(fn ConstructionScript
  (|CallParentFunction))