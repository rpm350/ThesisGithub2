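; Audio log interactable that plays its recording and raises a subtitle flag when possessed.
; Tick runs the parent logic, then polls the AudioLog component: if idle and Possessed is set, it starts playback from the beginning, sets ShowSubstitle and consumes Possessed.
; When idle and not possessed, it clears both flags, so the subtitle flag drops after playback ends.
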(event EventBeginPlay)

(event Collision|EventActorBeginOverlap
  (params (OtherActor :type Actor%20Object%20Reference)))

(event EventTick
  (params (DeltaSeconds :type Float%20%28single-precision%29))
  (bind _audiolog (Variables|Default|GetaudioLog))
  (|CallParentFunction DeltaSeconds)
  (if (Audio|Components|Audio|IsPlaying _audiolog)
    (if (not (Audio|Components|Audio|IsPlaying (Variables|Default|GetaudioLog))) :!label _label
      (Variables|Default|Setpossessed false)
      (Variables|Default|SetshowSubstitle false))
    (elif (Variables|Default|Getpossessed)
      (Variables|Default|SetshowSubstitle true)
      (Audio|Components|Audio|Play _audiolog 0.0)
      (Variables|Default|Setpossessed false)
      (else
        (goto _label)))))

(fn ConstructionScript
  (|CallParentFunction))