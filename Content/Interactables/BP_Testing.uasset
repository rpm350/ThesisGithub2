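; Test pawn in the Interactables folder that experiments with input-driven mesh rotation.
; On BeginPlay, a RotatingMovement component takes StaticMesh1 as its updated component.
; Turn input sets StaticMesh's relative yaw opposite to the axis sign, scaled by magnitude rather than accumulated, with pitch and roll copied from the actor.
; LookUp feeds controller pitch, while alternative yaw and actor-rotation logic is left unconnected.
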(event EventBeginPlay
  (Components|Movement|SetUpdatedComponent (Variables|Default|GetRotatingMovement) (Variables|Default|GetStaticMesh1)))

(event Collision|EventActorBeginOverlap
  (params (OtherActor :type Actor%20Object%20Reference)))

(event EventTick
  (params (DeltaSeconds :type Float%20%28single-precision%29))
  (|CallParentFunction DeltaSeconds) ; This node is disabled and will not be called.\nDrag off pins to build functionality.
)

(event Input|AxisEvents|InputAxisLookUp
  (params (AxisValue :type Float%20%28single-precision%29))
  (Pawn|Input|AddControllerPitchInput AxisValue))

(event Input|AxisEvents|InputAxisTurn
  (params (AxisValue :type Float%20%28single-precision%29))
  (bind _returnvalue (Transformation|GetActorRotation))
  (bind _returnvalue_2 (Transformation|GetActorRotation))
  (bind _returnvalue_3 (* AxisValue 0.05))
  (if (> AxisValue 0.0)
    (Transformation|SetRelativeRotation (Variables|Default|GetStaticMesh) (Math|Rotator|MakeRotator (.roll _returnvalue) (.pitch _returnvalue) (Math|Float|Lerp 0.0 -3.6e+02 _returnvalue_3)) false false)
    (else
      (Transformation|SetRelativeRotation (Variables|Default|GetStaticMesh) (Math|Rotator|MakeRotator (.roll _returnvalue_2) (.pitch _returnvalue_2) (Math|Float|Lerp 0.0 3.6e+02 (Math|Float|Absolute(Float) _returnvalue_3))) false false))))

(fn ConstructionScript
  (|CallParentFunction))