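; BP_OfficeFan is an interactable office fan that shoves an office chandelier to break glass.
; Overlapping a BP_OfficeChandelier stores it and arms the fan, with nothing in the file disarming it.
; The Perform input then plays audio, reapplies the rotating movement target and applies a large force to a chandelier skeletal bone.
; After a short delay, it plays a breaking sound and damages the linked glass's destructible component.
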(event Collision|EventActorBeginOverlap
  (params (OtherActor :type Actor%20Object%20Reference))
  (bind _asbp_office_chandelier (Utilities|Casting|CastToBP_OfficeChandelier OtherActor))
  (Variables|Default|SetreadyToPush true)
  (Variables|Default|SetmyChandelier _asbp_office_chandelier))

(event EventBeginPlay
  (Components|Movement|SetUpdatedComponent (Variables|Default|GetRotatingMovement) (Variables|Default|GetStaticMesh1)))

(event Input|ActionEvents|InputActionPerform
  (params (Key :type Key%20Structure))
  (bind _myglasstobreak (Variables|Default|GetmyGlassToBreak))
  (bind _rootcomponent (Variables|/Script/Engine.Actor|GetRootComponent _myglasstobreak))
  (bind _returnvalue (Transformation|GetWorldLocation _rootcomponent))
  (:Pressed
    (if (Variables|Default|GetreadyToPush)
      (Audio|Components|Audio|Play (Variables|Default|GetAudio) 0.0)
      (Components|Movement|SetUpdatedComponent (Variables|Default|GetRotatingMovement) (Variables|Default|GetStaticMesh1))
      (bind _asbp_office_chandelier (Utilities|Casting|CastToBP_OfficeChandelier (Variables|Default|GetmyChandelier)))
      (Utilities|IsValid "/Game/Interactables/PossesedObjects/Chandelier/BP_OfficeChandelier.BP_OfficeChandelier"
        (:Is%20Valid
          (Physics|AddForce (Variables|/Game/Interactables/PossesedObjects/Chandelier/BP_OfficeChandelier.BP_OfficeChandelier_C|GetSkeletalMesh _asbp_office_chandelier) "-30000000.000000,0.000000, 0" "CATRig10Bone001" false)
          (Utilities|FlowControl|Delay 0.2)
          (Utilities|IsValid _myglasstobreak
            (:Is%20Valid
              (Audio|Components|Audio|Play (Variables|Default|GetbreakGlass) 0.0)
              (Class|DestructibleComponent|ApplyDamage (Variables|/Script/ApexDestruction.DestructibleActor|GetDestructibleComponent _myglasstobreak) 1.0 _returnvalue _returnvalue 2.0))))))))

(fn ConstructionScript
  (|CallParentFunction))