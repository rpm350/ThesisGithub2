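; BP_SecurityCam is a security camera that plays a looping-style noise while the player controls it as their character.
; Each Tick it casts player character 0 to BP_SecurityCam, starting Sound if that is this camera and stopping it if the cast fails.
; Unconnected thermal-vision logic, which never runs, would swap target mesh materials to infrared and back.
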(event EventBeginPlay
  (|CallParentFunction))

(event Collision|EventActorBeginOverlap
  (params (OtherActor :type Actor%20Object%20Reference)))

(event EventTick
  (params (DeltaSeconds :type Float%20%28single-precision%29))
  (bind _sound (Variables|Default|Getsound))
  (bind _sound_2 (Variables|Default|Getsound))
  (|CallParentFunction DeltaSeconds)
  (bind _asbp_security_cam (Utilities|Casting|CastToBP_SecurityCam (Game|GetPlayerCharacter 0))
    (:then
      ;[1 1 1] play security cam noise
      (if (== _asbp_security_cam self)
        (if (not (Audio|Components|Audio|IsPlaying _sound_2))
          (Audio|Components|Audio|Play _sound_2 0.0))))
    (:CastFailed
      ;[1 1 1] Stop playing security cam noise
      (if (Audio|Components|Audio|IsPlaying _sound)
        (Audio|Components|Audio|Stop _sound)))))

(fn ConstructionScript
  (|CallParentFunction))