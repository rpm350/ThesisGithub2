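; Security camera that the player can control, running on top of parent class logic.
; Each tick it checks whether the player character is a BP_SecurityCam03, clamps view yaw if so, and plays camera noise when it is this instance.
; Otherwise it restores the yaw limits once and stops the noise.
; Thermal-vision material swaps and their reset on target actors are present but never run.
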(event EventBeginPlay
  (|CallParentFunction))

(event Collision|EventActorBeginOverlap
  (params (OtherActor :type Actor%20Object%20Reference)))

(event EventTick
  (params (DeltaSeconds :type Float%20%28single-precision%29))
  (bind _returnvalue (Game|GetPlayerCameraManager 0))
  (bind _returnvalue_2 (Game|GetPlayerCameraManager 0))
  (bind _sound (Variables|Default|Getsound))
  (bind _sound_2 (Variables|Default|Getsound))
  (|CallParentFunction DeltaSeconds)
  (bind _asbp_security_cam_03 (Utilities|Casting|CastToBP_SecurityCam03 (Game|GetPlayerCharacter 0))
    (:then
      ;[1 1 1] Handle Clamping the Camera
      (Variables|Default|SetsetClamp true)
      (Variables|/Script/Engine.PlayerCameraManager|SetViewYawMin _returnvalue -3.5e+02)
      (Variables|/Script/Engine.PlayerCameraManager|SetViewYawMax _returnvalue 1.7e+02)
      ;[1 1 1] play security cam noise
      (if (== _asbp_security_cam_03 self)
        (if (not (Audio|Components|Audio|IsPlaying _sound_2))
          (Audio|Components|Audio|Play _sound_2 0.0))))
    (:CastFailed
      (if (Variables|Default|GetsetClamp)
        (Variables|Default|SetsetClamp false)
        (Variables|/Script/Engine.PlayerCameraManager|SetViewYawMin _returnvalue_2 0.0)
        (Variables|/Script/Engine.PlayerCameraManager|SetViewYawMax _returnvalue_2 359.0))
      ;[1 1 1] Stop playing security cam noise
      (if (Audio|Components|Audio|IsPlaying _sound)
        (Audio|Components|Audio|Stop _sound)))))

(fn ConstructionScript
  (|CallParentFunction))