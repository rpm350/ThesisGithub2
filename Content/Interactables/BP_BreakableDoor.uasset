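; BP_BreakableDoor is an interactable door whose glass can be smashed by an office chandelier or a hammer.
; Its Box overlap breaks the glass on any chandelier contact, or on hammer contact only during a swing or back swing.
; Breaking destroys the referenced MyGlass actor, if still valid, and plays GlassBreakSound.
; A leftover debug string prints on every overlap.
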(event OnComponentBeginOverlap(Box)
  (params (OverlappedComponent :type Primitive%20Component%20Object%20Reference) (OtherActor :type Actor%20Object%20Reference) (OtherComp :type Primitive%20Component%20Object%20Reference) (OtherBodyIndex :type Integer) (bFromSweep :type Boolean) (SweepResult :type Hit%20Result%20Structure%20%28by%20ref%29))
  (bind _myglass (Variables|Default|GetmyGlass))
  (Development|PrintString "JDKSJEKJNWSOEUNFS")
  (Utilities|Casting|CastToBP_OfficeChandelier OtherActor
    (:then
      (Utilities|IsValid _myglass :!label _label
        (:Is%20Valid
          (Actor|DestroyActor _myglass)
          (Audio|Components|Audio|Play (Variables|Default|GetglassBreak_sound) 0.0))))
    (:CastFailed
      (bind _asbp_hammer (Utilities|Casting|CastToBP_Hammer OtherActor))
      (if (or (Variables|/Game/Interactables/BP_Hammer.BP_Hammer_C|Getswing _asbp_hammer) (Variables|/Game/Interactables/BP_Hammer.BP_Hammer_C|GetswingBack _asbp_hammer))
        (goto _label)))))

(event EventBeginPlay)

(event Collision|EventActorBeginOverlap
  (params (OtherActor :type Actor%20Object%20Reference)))

(event EventTick
  (params (DeltaSeconds :type Float%20%28single-precision%29)))

(fn ConstructionScript)