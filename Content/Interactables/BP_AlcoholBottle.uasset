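; BP_AlcoholBottle is a player-controlled bottle, built on Ball Template movement, that tips over to pour a one-time puddle of alcohol or water.
; Perform starts a Tick-driven RInterpTo swing to the pour rotation and back, while mouse look turns the camera and holds the mesh rotation when idle.
; At full swing it reveals its child BP_Puddle, enables trailing, plays fall and liquid sounds, and triggers any NPC whiskey reaction volume.
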(event EventBeginPlay
  (bind _asbp_puddle (Utilities|Casting|CastToBP_Puddle (Variables|/Script/Engine.ChildActorComponent|GetChildActor (Variables|Default|Getpuddle))))
  (bind _output_get (Variables|Default|SetmyPuddle _asbp_puddle))
  (Variables|/Game/Interactables/BP_Puddle.BP_Puddle_C|SetsourcePuddle _output_get true)
  (Default|SetSourcePuddle _output_get)
  (Variables|Default|SetstartingCamRot (Transformation|GetWorldRotation (Variables|Default|GetFollowCamera)))
  (if (Variables|Default|GetisWater)
    (Rendering|Material|SetMaterial (Variables|/Game/Interactables/BP_Puddle.BP_Puddle_C|GetPuddle _asbp_puddle) 0 "/Game/StarterContent/Materials/M_Water.M_Water")))

(event Collision|EventActorBeginOverlap
  (params (OtherActor :type Actor%20Object%20Reference)))

(event EventTick
  (params (DeltaSeconds :type Float%20%28single-precision%29))
  (bind _mynpcreactionvolume (Variables|Default|GetmyNPCReactionVolume))
  (bind _puddle (Variables|Default|Getpuddle))
  (|CallParentFunction DeltaSeconds)
  (Transformation|SetWorldRotation (Variables|Default|Getpuddle) "0, 0, 0" false false)
  (if (Variables|Default|Getswing)
    (if (Math|Rotator|Equal(Rotator) (Variables|Default|GetmoveRot) (Variables|Default|GetswingRotation) 0.1)
      (Variables|Default|SetswingBack true)
      (Variables|Default|Setswing false)
      (if (not (Variables|Default|Getpoured))
        (if (not (Variables|/Game/Interactables/BP_Puddle.BP_Puddle_C|GetcanTrail (Variables|Default|GetmyPuddle)))
          (Variables|/Game/Interactables/BP_Puddle.BP_Puddle_C|SetcanTrail (Variables|Default|GetmyPuddle) true)
          (Rendering|SetVisibility _puddle true false)
          (bind _asbp_puddle (Utilities|Casting|CastToBP_Puddle (Variables|/Script/Engine.ChildActorComponent|GetChildActor (Variables|Default|Getpuddle))))
          (if (Variables|Default|GetisWater)
            (Rendering|Material|SetMaterial (Variables|/Game/Interactables/BP_Puddle.BP_Puddle_C|Getround%20puddle _asbp_puddle) 0 "/Game/StarterContent/Materials/M_Water.M_Water"))
          (Transformation|SetWorldRotation _puddle "0, 0, 0" false false)
          (Audio|Components|Audio|Play (Variables|Default|GetbottleFall_sound) 0.0)
          (Audio|Components|Audio|Play (Variables|Default|Getliquid_sound) 0.0)
          (Variables|Default|Setpoured true)
          (Utilities|IsValid _mynpcreactionvolume
            (:Is%20Valid
              (Default|ReactWhiskey _mynpcreactionvolume)))))
      (else
        (bind _output_get (Variables|Default|SetmoveRot (Math|Interpolation|RInterpTo (Variables|Default|GetmoveRot) (Variables|Default|GetswingRotation) DeltaSeconds 5.0)))
        (Transformation|SetActorRotation _output_get)))
    (elif (Variables|Default|GetswingBack)
      (if (Math|Rotator|Equal(Rotator) (Variables|Default|GetmoveRot) (Variables|Default|GetbaseRotation) 0.1)
        (Variables|Default|SetswingBack false)
        (Variables|Default|SetmoveRot "0,180.000000, 0")
        (else
          (bind _output_get_2 (Variables|Default|SetmoveRot (Math|Interpolation|RInterpTo (Variables|Default|GetmoveRot) (Variables|Default|GetbaseRotation) DeltaSeconds 5.0)))
          (Transformation|SetActorRotation _output_get_2))))))

(event Input|ActionEvents|InputActionPerform
  (params (Key :type Key%20Structure))
  (bind _mypuddle (Variables|Default|GetmyPuddle))
  (:Pressed
    (if (not (Variables|Default|Getpoured))
      (Variables|Default|Setswing true)
      (Variables|/Game/Interactables/BP_Puddle.BP_Puddle_C|SetsourcePuddle _mypuddle true)
      (Default|SetSourcePuddle _mypuddle))))

(event Input|AxisEvents|InputAxisLookUp
  (params (AxisValue :type Float%20%28single-precision%29))
  ;[1 1 1] Mouse input - overriding Ball Template's movement
  (Pawn|Input|AddControllerPitchInput AxisValue)
  (Transformation|SetWorldRotation (Variables|Default|GetStaticMesh) (Variables|Default|GetmoveRot) false false))

(event Input|AxisEvents|InputAxisTurn
  (params (AxisValue :type Float%20%28single-precision%29))
  ;[1 1 1] Mouse input - overriding Ball Template's movement
  (Pawn|Input|AddControllerYawInput AxisValue)
  (if (not (or (Variables|Default|Getswing) (Variables|Default|GetswingBack)))
    (Transformation|SetWorldRotation (Variables|Default|GetStaticMesh) (Variables|Default|GetmoveRot) false false)))

(fn ConstructionScript
  (|CallParentFunction))