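; BP_CartWheel is a player-controllable pawn with standard movement and look input, with no cartwheel-specific logic in its graphs.
; Move axes drive movement input along the actor's forward and right vectors, or the FollowCamera's when a head-mounted display is enabled.
; Turn and look axes feed controller yaw and pitch directly, while rate variants scale by base rates and frame delta time.
; Tick, BeginPlay, overlap and construction script add no behavior.
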(event EventBeginPlay)

(event Collision|EventActorBeginOverlap
  (params (OtherActor :type Actor%20Object%20Reference)))

(event EventTick
  (params (DeltaSeconds :type Float%20%28single-precision%29))
  (|CallParentFunction DeltaSeconds) ; This node is disabled and will not be called.\nDrag off pins to build functionality.
)

(event Input|AxisEvents|InputAxisTurn
  (params (AxisValue :type Float%20%28single-precision%29))
  ;[1 1 1] turning
  (Pawn|Input|AddControllerYawInput AxisValue))

(event Input|AxisEvents|InputAxisLookUp
  (params (AxisValue :type Float%20%28single-precision%29))
  ;[1 1 1] turning
  (Pawn|Input|AddControllerPitchInput AxisValue))

(event Input|AxisEvents|InputAxisMoveForward
  (params (AxisValue :type Float%20%28single-precision%29))
  ;[1 1 1] movement
  (Pawn|Input|AddMovementInput (select (Class|HeadMountedDisplayFunctionLibrary|IsHeadMountedDisplayEnabled) (Math|Vector|GetForwardVector (Variables|Default|GetFollowCamera)) (Transformation|GetActorForwardVector)) AxisValue false))

(event Input|AxisEvents|InputAxisMoveRight
  (params (AxisValue :type Float%20%28single-precision%29))
  ;[1 1 1] movement
  (Pawn|Input|AddMovementInput (select (Class|HeadMountedDisplayFunctionLibrary|IsHeadMountedDisplayEnabled) (Math|Vector|GetRightVector (Variables|Default|GetFollowCamera)) (Transformation|GetActorRightVector)) AxisValue false))

(event Input|AxisEvents|InputAxisTurnRate
  (params (AxisValue :type Float%20%28single-precision%29))
  ;[1 1 1] turn
  (Pawn|Input|AddControllerYawInput (* AxisValue (Variables|Default|GetBaseTurnRate) (Utilities|Time|GetWorldDeltaSeconds))))

(event Input|AxisEvents|InputAxisLookUpRate
  (params (AxisValue :type Float%20%28single-precision%29))
  ;[1 1 1] turn
  (Pawn|Input|AddControllerPitchInput (* AxisValue (Variables|Default|GetBaseLookUpRate) (Utilities|Time|GetWorldDeltaSeconds))))

(fn ConstructionScript
  (|CallParentFunction))