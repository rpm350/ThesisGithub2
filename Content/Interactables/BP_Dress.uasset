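; BP_Dress is a wheeled, input-driven interactable that moves along its starting forward axis and leaves puddle trails.
; Wheel overlap events with trailable source puddles start per-wheel tracking, with one trigger on end overlap.
; Tick spawns BP_Puddle below each tracked wheel after PuddleDiam of X/Y movement, up to a maximum, playing sound on alternate counts.
; Wheel names and timers are cross-wired between corners.
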(event OnComponentBeginOverlap(wheel_BR)
  (params (OverlappedComponent :type Primitive%20Component%20Object%20Reference) (OtherActor :type Actor%20Object%20Reference) (OtherComp :type Primitive%20Component%20Object%20Reference) (OtherBodyIndex :type Integer) (bFromSweep :type Boolean) (SweepResult :type Hit%20Result%20Structure%20%28by%20ref%29))
  ;[1 1 1] Hit a puddle? Need to track?
  (bind _asbp_puddle (Utilities|Casting|CastToBP_Puddle OtherActor))
  (if (Variables|/Game/Interactables/BP_Puddle.BP_Puddle_C|GetcanTrail _asbp_puddle)
    (if (Variables|/Game/Interactables/BP_Puddle.BP_Puddle_C|GetsourcePuddle _asbp_puddle)
      (if (or (>= (Variables|Default|GetFRTimer) (Variables|Default|GetspawnPuddleMax)) (== (Variables|Default|GetFRTimer) 0))
        (Variables|Default|SettrackingFR true)
        (Variables|Default|SetFRTimer 0)))))

(event OnComponentBeginOverlap(wheel_FL)
  (params (OverlappedComponent :type Primitive%20Component%20Object%20Reference) (OtherActor :type Actor%20Object%20Reference) (OtherComp :type Primitive%20Component%20Object%20Reference) (OtherBodyIndex :type Integer) (bFromSweep :type Boolean) (SweepResult :type Hit%20Result%20Structure%20%28by%20ref%29))
  ;[1 1 1] Hit a puddle? Need to track?
  (bind _asbp_puddle (Utilities|Casting|CastToBP_Puddle OtherActor))
  (if (Variables|/Game/Interactables/BP_Puddle.BP_Puddle_C|GetcanTrail _asbp_puddle)
    (if (Variables|/Game/Interactables/BP_Puddle.BP_Puddle_C|GetsourcePuddle _asbp_puddle)
      (if (or (>= (Variables|Default|GetFLTimer) (Variables|Default|GetspawnPuddleMax)) (== (Variables|Default|GetFLTimer) 0))
        (Variables|Default|SettrackingFL true)
        (Variables|Default|SetFLTimer 0)))))

(event OnComponentBeginOverlap(wheel_BL)
  (params (OverlappedComponent :type Primitive%20Component%20Object%20Reference) (OtherActor :type Actor%20Object%20Reference) (OtherComp :type Primitive%20Component%20Object%20Reference) (OtherBodyIndex :type Integer) (bFromSweep :type Boolean) (SweepResult :type Hit%20Result%20Structure%20%28by%20ref%29))
  ;[1 1 1] Hit a puddle? Need to track?
  (bind _asbp_puddle (Utilities|Casting|CastToBP_Puddle OtherActor))
  (if (Variables|/Game/Interactables/BP_Puddle.BP_Puddle_C|GetcanTrail _asbp_puddle)
    (if (Variables|/Game/Interactables/BP_Puddle.BP_Puddle_C|GetsourcePuddle _asbp_puddle)
      (if (or (>= (Variables|Default|GetBRTimer) (Variables|Default|GetspawnPuddleMax)) (== (Variables|Default|GetBRTimer) 0))
        (Variables|Default|SettrackingBR true)
        (Variables|Default|SetBRTimer 0)))))

(event OnComponentEndOverlap(wheel_FL)
  (params (OverlappedComponent :type Primitive%20Component%20Object%20Reference) (OtherActor :type Actor%20Object%20Reference) (OtherComp :type Primitive%20Component%20Object%20Reference) (OtherBodyIndex :type Integer))
  ;[1 1 1] Hit a puddle? Need to track?
  (bind _asbp_puddle (Utilities|Casting|CastToBP_Puddle OtherActor))
  (if (Variables|/Game/Interactables/BP_Puddle.BP_Puddle_C|GetcanTrail _asbp_puddle)
    (if (Variables|/Game/Interactables/BP_Puddle.BP_Puddle_C|GetsourcePuddle _asbp_puddle)
      (if (or (>= (Variables|Default|GetBLTimer) (Variables|Default|GetspawnPuddleMax)) (== (Variables|Default|GetBLTimer) 0))
        (Variables|Default|SettrackingBL true)
        (Variables|Default|SetBLTimer 0)))))

(event EventTick
  (params (DeltaSeconds :type Float%20%28single-precision%29))
  (bind _trunkwheel_rl (Variables|Default|GetTrunkWheel_RL))
  (bind _trunkwheel_rl_2 (Variables|Default|GetTrunkWheel_RL))
  (bind _trunkwheel_fl (Variables|Default|GetTrunkWheel_FL))
  (bind _trunkwheel_fl_2 (Variables|Default|GetTrunkWheel_FL))
  (bind _trunkwheel_rr (Variables|Default|GetTrunkWheel_RR))
  (bind _trunkwheel_rr_2 (Variables|Default|GetTrunkWheel_RR))
  (bind _trunkwheel_fr (Variables|Default|GetTrunkWheel_FR))
  (bind _trunkwheel_fr_2 (Variables|Default|GetTrunkWheel_FR))
  (bind _returnvalue (Transformation|GetWorldLocation _trunkwheel_fr))
  (bind _returnvalue_2 (Transformation|GetWorldLocation _trunkwheel_rr))
  (bind _returnvalue_3 (Transformation|GetWorldLocation _trunkwheel_rl))
  (bind _returnvalue_4 (Transformation|GetWorldLocation _trunkwheel_fl))
  (bind _returnvalue_5 (Transformation|GetWorldLocation _trunkwheel_rr_2))
  (bind _returnvalue_6 (Transformation|GetWorldLocation _trunkwheel_rl_2))
  (bind _returnvalue_7 (Transformation|GetWorldLocation _trunkwheel_fl_2))
  (bind _returnvalue_8 (Transformation|GetWorldLocation _trunkwheel_fr_2))
  (bind (_x _y _z) (Math|Vector|BreakVector _returnvalue_3))
  (bind (_x_2 _y_2 _z_2) (Math|Vector|BreakVector _returnvalue_4))
  (bind (_x_3 _y_3 _z_3) (Math|Vector|BreakVector _returnvalue_5))
  (bind (_x_4 _y_4 _z_4) (Math|Vector|BreakVector _returnvalue))
  ;[1 1 1] Check if need to trail the puddle
  (if (Variables|Default|GettrackingBR)
    (if (<= (Variables|Default|GetBRTimer) (Variables|Default|GetspawnPuddleMax))
      (bind _movedfarenoughtospawn (CallFunction|AbsVal _returnvalue_6 (Variables|Default|GetBRprevLoc)))
      (if _movedfarenoughtospawn
        (Game|SpawnActorfromClass "/Game/Interactables/BP_Puddle.BP_Puddle_C" (Math|Transform|MakeTransform (Math|Vector|MakeVector _x _y (- _z (Variables|Default|GetpuddleHeightFromGround)))) "Undefined" 0 0)
        (if (== (Math|Integer|%(Integer) (Variables|Default|GetBRTimer) 2) 0)
          (Audio|Components|Audio|Play (Variables|Default|Getpuddle_sound) 0.0))
        (Variables|Default|SetBRprevLoc _returnvalue_6)
        (Variables|Default|SetBRTimer (+ (Variables|Default|GetBRTimer) 1)))))
  (if (Variables|Default|GettrackingBL)
    (if (<= (Variables|Default|GetBLTimer) (Variables|Default|GetspawnPuddleMax))
      (bind _movedfarenoughtospawn_2 (CallFunction|AbsVal _returnvalue_7 (Variables|Default|GetBLprevLoc)))
      (if _movedfarenoughtospawn_2
        (Game|SpawnActorfromClass "/Game/Interactables/BP_Puddle.BP_Puddle_C" (Math|Transform|MakeTransform (Math|Vector|MakeVector _x_2 _y_2 (- _z_2 (Variables|Default|GetpuddleHeightFromGround)))) "Undefined" 0 0)
        (if (== (Math|Integer|%(Integer) (Variables|Default|GetFLTimer) 2) 0)
          (Audio|Components|Audio|Play (Variables|Default|Getpuddle_sound) 0.0))
        (Variables|Default|SetBLprevLoc _returnvalue_7)
        (Variables|Default|SetBLTimer (+ (Variables|Default|GetFLTimer) 1)))))
  (if (Variables|Default|GettrackingFR)
    (if (<= (Variables|Default|GetFRTimer) (Variables|Default|GetspawnPuddleMax))
      (bind _movedfarenoughtospawn_3 (CallFunction|AbsVal _returnvalue_2 (Variables|Default|GetFRprevLoc)))
      (if _movedfarenoughtospawn_3
        (Game|SpawnActorfromClass "/Game/Interactables/BP_Puddle.BP_Puddle_C" (Math|Transform|MakeTransform (Math|Vector|MakeVector _x_3 _y_3 (- _z_3 (Variables|Default|GetpuddleHeightFromGround)))) "Undefined" 0 0)
        (if (== (Math|Integer|%(Integer) (Variables|Default|GetFRTimer) 2) 0)
          (Audio|Components|Audio|Play (Variables|Default|Getpuddle_sound) 0.0))
        (Variables|Default|SetFRprevLoc _returnvalue_2)
        (Variables|Default|SetFRTimer (+ (Variables|Default|GetFRTimer) 1)))))
  (if (Variables|Default|GettrackingFL)
    (if (<= (Variables|Default|GetFLTimer) (Variables|Default|GetspawnPuddleMax))
      (bind _movedfarenoughtospawn_4 (CallFunction|AbsVal _returnvalue_8 (Variables|Default|GetFLprevLoc)))
      (if _movedfarenoughtospawn_4
        (Game|SpawnActorfromClass "/Game/Interactables/BP_Puddle.BP_Puddle_C" (Math|Transform|MakeTransform (Math|Vector|MakeVector _x_4 _y_4 (- _z_4 (Variables|Default|GetpuddleHeightFromGround)))) "Undefined" 0 0)
        (if (== (Math|Integer|%(Integer) (Variables|Default|GetFLTimer) 2) 0)
          (Audio|Components|Audio|Play (Variables|Default|Getpuddle_sound) 0.0))
        (Variables|Default|SetFLprevLoc _returnvalue_8)
        (Variables|Default|SetFLTimer (+ (Variables|Default|GetFRTimer) 1))
        (else
          (|CallParentFunction DeltaSeconds :!label _label)))
      (else
        (goto _label)))
    (else
      (goto _label))))

(event Collision|EventActorBeginOverlap
  (params (OtherActor :type Actor%20Object%20Reference)))

(event EventBeginPlay
  ;[1 1 1] Begin Play
  (Variables|Default|Setforward (Transformation|GetActorForwardVector))
  (Variables|Default|SetBRprevLoc (Transformation|GetWorldLocation (Variables|Default|GetTrunkWheel_RL)))
  (Variables|Default|SetFRprevLoc (Transformation|GetWorldLocation (Variables|Default|GetTrunkWheel_RR)))
  (Variables|Default|SetBLprevLoc (Transformation|GetWorldLocation (Variables|Default|GetTrunkWheel_FL)))
  (Variables|Default|SetFLprevLoc (Transformation|GetWorldLocation (Variables|Default|GetTrunkWheel_FR))))

(event Input|AxisEvents|InputAxisMoveForward
  (params (AxisValue :type Float%20%28single-precision%29))
  ;[1 1 1] movement
  (Pawn|Input|AddMovementInput (Variables|Default|Getforward) AxisValue false))

(fn ConstructionScript
  (|CallParentFunction))

(fn AbsVal
  (params (currentPos :type Vector) (prevPos :type Vector))
  (bind (_x _y) (Math|Vector|BreakVector prevPos))
  (bind (_x_2 _y_2) (Math|Vector|BreakVector currentPos))
  (bind _puddlediam (Variables|Default|GetpuddleDiam))
  (Variables|Default|SetabsVal_x false)
  (Variables|Default|SetabsVal_z false)
  (if (< _x_2 (+ _x _puddlediam))
    ;[1 1 1] Change is too small
    (Variables|Default|SetabsVal_x false)
    (if (> _x_2 (- _x _puddlediam))
      (Variables|Default|SetabsVal_x false)
      (if (< _y_2 (+ _y _puddlediam))
        (Variables|Default|SetabsVal_z false)
        (if (> _y_2 (- _y _puddlediam))
          (Variables|Default|SetabsVal_z false)
          (return false)
          (else
            (Variables|Default|SetabsVal_z true)))
        (else
          (Variables|Default|SetabsVal_z true)))
      (return true)
      (else
        (Variables|Default|SetabsVal_x true)))
    (else
      (Variables|Default|SetabsVal_x true)))
  (return true))