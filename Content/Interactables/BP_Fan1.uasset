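; BP_Fan1 is a spinning fan interactable that blows a hanging chain sax away when it overlaps.
; A RotatingMovement component spins StaticMesh1.
; Overlap with BP_ChainSax plays the fan sound and applies a large negative-Y force to one skeletal bone.
; It also carries Turn and LookUp axis handlers that set camera yaw limits and feed controller look, plus disconnected chandelier-cast and impulse nodes.
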(event Collision|EventActorBeginOverlap
  (params (OtherActor :type Actor%20Object%20Reference))
  (bind _asbp_chain_sax (Utilities|Casting|CastToBP_ChainSax OtherActor))
  (Audio|Components|Audio|Play (Variables|Default|Getfan_sound) 0.0)
  (Physics|AddForce (Variables|/Game/Interactables/PossesedObjects/ChainSaxophone/BP_ChainSax.BP_ChainSax_C|GetSkeletalMesh _asbp_chain_sax) "0,-90000000.000000, 0" "CATRig10Bone001" false))

(event EventBeginPlay
  (Components|Movement|SetUpdatedComponent (Variables|Default|GetRotatingMovement) (Variables|Default|GetStaticMesh1)))

(event Input|AxisEvents|InputAxisLookUp
  (params (AxisValue :type Float%20%28single-precision%29))
  (Pawn|Input|AddControllerPitchInput AxisValue))

(event Input|AxisEvents|InputAxisTurn
  (params (AxisValue :type Float%20%28single-precision%29))
  (bind _returnvalue (Game|GetPlayerCameraManager 0))
  (Variables|/Script/Engine.PlayerCameraManager|SetViewYawMin _returnvalue 55.0)
  (Variables|/Script/Engine.PlayerCameraManager|SetViewYawMax _returnvalue 0.0)
  (Pawn|Input|AddControllerYawInput (* AxisValue 0.35)))

(fn ConstructionScript
  (|CallParentFunction))