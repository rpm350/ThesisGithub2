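; BP_SawControl is an interactable control that triggers a linked saw's cut once.
; The Perform input press calls Cut on the MySaw reference and sets a Done flag that blocks further presses.
; The same press swaps the mesh material to a pulsing red light and plays the Button component from the start.
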(event EventBeginPlay
  (|CallParentFunction) ; This node is disabled and will not be called.\nDrag off pins to build functionality.
)

(event Collision|EventActorBeginOverlap
  (params (OtherActor :type Actor%20Object%20Reference)))

(event EventTick
  (params (DeltaSeconds :type Float%20%28single-precision%29))
  (|CallParentFunction DeltaSeconds))

(event Input|ActionEvents|InputActionPerform
  (params (Key :type Key%20Structure))
  (:Pressed
    (if (not (Variables|Default|Getdone))
      (Default|Cut (Variables|Default|GetmySaw))
      (Variables|Default|Setdone true)
      (Rendering|Material|SetMaterial (Variables|Default|GetStaticMesh) 0 "/Game/Materials/PulsingLight/MAT_RedLightPulse.MAT_RedLightPulse")
      (Audio|Components|Audio|Play (Variables|Default|Getbutton) 0.0))))

(fn ConstructionScript
  (|CallParentFunction))